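; Elevator actor with a floor button that moves a platform up or down when the player character enters its trigger box.
; Overlap passes a DoOnce gate, posts a Wwise sound and presses the button via timeline, then a FlipFlop plays or reverses the platform timeline scaled by TargetHeight.
; Leaving while IsMoving is false raises the button and resets the gate after a delay.
; A duplicate FlipFlop/timeline chain is never run.
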(event `self.Box.OnComponentBeginOverlap`
  (params (OverlappedComponent :type "PrimitiveComponent Object Reference") (OtherActor :type "Actor Object Reference") (OtherComp :type "PrimitiveComponent Object Reference") (OtherBodyIndex :type Integer) (bFromSweep :type Boolean) (SweepResult :type "HitResult Structure (by ref)"))
  (bind _elevatorbutton (`self.ElevatorButton`))
  (if (== OtherActor (`/Game/Blueprints/BFL_CommonFunctions.GetPlayerCharacterRef`))
    (`/Engine/EditorBlueprintResources/StandardMacros.DoOnce` false :!label _label
      (:`Completed`
        (`AkGameplayStatics.PostEvent` "/Game/WwiseAudio/PedButtons.PedButtons")
        (bind (_direction _alpha) (`Timeline|ButtonTL`)
          (:`Update`
            (`SceneComponent.K2_SetRelativeLocation` _elevatorbutton (`KismetMathLibrary.VInterpTo` (`SceneComponent.RelativeLocation` _elevatorbutton) (0.0 0.0 6.5) _alpha) false false))
          (:`Finished`
            (set `self.isMoving?` true)
            (`/Engine/EditorBlueprintResources/StandardMacros.FlipFlop`
              (:`A`
                (bind (_direction_2 _elevatorlocation) (`Timeline|Timeline` :!label _label_2)
                  (:`Update`
                    (`SceneComponent.K2_SetRelativeLocation` (`self.ElevatorPlatform`) (* _elevatorlocation (`KismetMathLibrary.MakeVector` 0.0 0.0 (`self.TargetHeight`))) false false))
                  (:`Finished`
                    (set `self.isMoving?` false))))
              (:`B`
                (goto _label_2 :!via `Reverse`)))))))))

(event `self.Box.OnComponentEndOverlap`
  (params (OverlappedComponent :type "PrimitiveComponent Object Reference") (OtherActor :type "Actor Object Reference") (OtherComp :type "PrimitiveComponent Object Reference") (OtherBodyIndex :type Integer))
  (bind _elevatorbutton (`self.ElevatorButton`))
  (if (== OtherActor (`/Game/Blueprints/BFL_CommonFunctions.GetPlayerCharacterRef`))
    (if (not (`self.isMoving?`))
      (bind (_direction _alpha) (`Timeline|ButtonReleaseTL`)
        (:`Update`
          (`SceneComponent.K2_SetRelativeLocation` _elevatorbutton (`KismetMathLibrary.VInterpTo` (`SceneComponent.RelativeLocation` _elevatorbutton) (0.0 0.0 11.5) _alpha) false false)
          (`KismetSystemLibrary.Delay` 1.0)
          (goto _label :!via `Reset`))))))

(event `Key|E`
  (params (Key :type "Key Structure")))

(fn `UserConstructionScript`)