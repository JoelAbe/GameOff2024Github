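; Checkpoint actor that saves the game when the player character overlaps its sphere.
; BeginPlay caches player references and starts a short timer that enables saving, so overlaps before it fires are ignored.
; On overlap it gathers character and world save data, passes both to the Jam game instance subsystem, then tells it to save.
; Debug prints report the save and the first unlockable-door entry.
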(event `self.ReceiveBeginPlay`
  (set `self.Player Controller Ref` (`/Game/Blueprints/BFL_CommonFunctions.GetPlayerControllerRef`))
  (set `self.Player Character Ref` (`/Game/Blueprints/BFL_CommonFunctions.GetPlayerCharacterRef`))
  (`KismetSystemLibrary.K2_SetTimerDelegate` (delegate `AllowSaving`) 3.0))

(event `AllowSaving`
  (set `self.AllowSave` true))

(event `self.Sphere.OnComponentBeginOverlap`
  (params (OverlappedComponent :type "PrimitiveComponent Object Reference") (OtherActor :type "Actor Object Reference") (OtherComp :type "PrimitiveComponent Object Reference") (OtherBodyIndex :type Integer) (bFromSweep :type Boolean) (SweepResult :type "HitResult Structure (by ref)"))
  (bind _returnvalue (subsystem `JamGameInstanceSubsystem`))
  (if (and (== OtherActor (`self.Player Character Ref`)) (`self.AllowSave`))
    (`KismetSystemLibrary.PrintString` "Save")
    (bind _returnvalue_2 (`JamPlayerCharacter.GetCharacterSaveData` (`self.Player Character Ref`)))
    (message `SaveGameInterface.SetPlayerSaveData` _returnvalue _returnvalue_2)
    (bind _returnvalue_3 (`self.GetWorldSaveData`))
    (message `SaveGameInterface.SetWorldSaveData` _returnvalue _returnvalue_3)
    (message `SaveGameInterface.SaveGameData` _returnvalue)
    (`KismetSystemLibrary.PrintString` (`KismetStringLibrary.Conv_BoolToString` (`|GetArrayItem` (`.UnlockableDoorsArray` (break `WorldSave` _returnvalue_3)))))))

(fn `UserConstructionScript`)