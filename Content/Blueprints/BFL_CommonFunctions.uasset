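; Blueprint function library of shorthand getters for the jam game's core player objects and master UI widget.
; The character, controller and player state getters each fetch index 0 and cast to the matching BP_Jam class.
; The master widget getter reads MasterWidgetRef from a player controller that is passed in, rather than looking one up itself.
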(fn `GetMasterWidgetRef`
  (params (PlayerControllerRef :type "/Game/Player/BP_JamPlayerController Object Reference"))
  (returns (MasterWidgetRef :type "/Game/UI/Common/Widgets/WB_MasterWidget Object Reference"))
  (return (`/Game/Player/BP_JamPlayerController.MasterWidgetRef` PlayerControllerRef)))

(fn `GetPlayerCharacterRef`
  (returns (PlayerCharacterRef :type "/Game/Player/BP_JamPlayerCharacter Object Reference"))
  (bind _asbp_jam_player_character (cast `/Game/Player/BP_JamPlayerCharacter` (`GameplayStatics.GetPlayerCharacter` null))
    (:`then`
      (return _asbp_jam_player_character))
    (:`CastFailed`
      (return _asbp_jam_player_character))))

(fn `GetPlayerControllerRef`
  (returns (PlayerControllerRef :type "/Game/Player/BP_JamPlayerController Object Reference"))
  (bind _asbp_jam_player_controller (cast `/Game/Player/BP_JamPlayerController` (`GameplayStatics.GetPlayerController` null))
    (:`then`
      (return _asbp_jam_player_controller))
    (:`CastFailed`
      (return _asbp_jam_player_controller))))

(fn `GetPlayerStateRef`
  (returns (PlayerStateRef :type "/Game/Player/BP_JamPlayerState Object Reference"))
  (bind _asbp_jam_player_state (cast `/Game/Player/BP_JamPlayerState` (`GameplayStatics.GetPlayerState` null))
    (:`then`
      (return _asbp_jam_player_state))
    (:`CastFailed`
      (return null))))