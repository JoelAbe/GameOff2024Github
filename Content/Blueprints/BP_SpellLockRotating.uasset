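; BP_SpellLockRotating is a spell lock that unlocks its linked door when hit by the required spell.
; Box overlaps check spell IDs from projectile, summoned companion or fire shotgun actors, then activate the crystal, play effects, and remove the box.
; The construction script chooses Niagara effects from the required ID.
; After a short BeginPlay delay, it restores state from save data and replays activation if already unlocked.
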(event `self.ReceiveBeginPlay`
  (`KismetSystemLibrary.Delay` 0.2)
  (bind _returnvalue (message `SaveGameInterface.GetSaveGameData` (subsystem `JamGameInstanceSubsystem`)))
  (`/Engine/EditorBlueprintResources/StandardMacros.IsValid` _returnvalue
    (:`Is Valid`
      (`self.SetStateFromSaveData` (`JamSaveGameObject.WorldData` _returnvalue))
      (`self.OnWorldLoad`))))

(event `OnWorldLoad`
  (if (`self.isActivated`)
    (`self.ActivateCrystal`)))

(event `self.Box.OnComponentBeginOverlap`
  (params (OverlappedComponent :type "PrimitiveComponent Object Reference") (OtherActor :type "Actor Object Reference") (OtherComp :type "PrimitiveComponent Object Reference") (OtherBodyIndex :type Integer) (bFromSweep :type Boolean) (SweepResult :type "HitResult Structure (by ref)"))
  (bind _linkeddoor (`self.LinkedDoor`))
  (if (not (`self.isActivated`))
    (bind _asmagic_projectile (cast `MagicProjectile` OtherActor)
      (:`then`
        (set `self.CastIndex` 0)
        (if (== (select `int` (`self.CastIndex`) :`0` (`.ID` (break `Spell` (`MagicProjectile.SpellData` _asmagic_projectile))) :`1` (`SummonedSpellDamageCompanion.SpellID` (stale _assummoned_spell_damage_companion)) :`2` (`/Game/Blueprints/Combat/BP_FireShotgun.SpellID` (stale _asbp_fire_shotgun))) (`self.RequiredIDToUnlockDoor`)) :!label _label
          (`/Engine/EditorBlueprintResources/StandardMacros.DoOnce` false
            (:`Completed`
              (`self.ActivateCrystal`)
              (`ActorComponent.Activate` (`self.UnlockedEffect`) false)
              (`/Engine/EditorBlueprintResources/StandardMacros.IsValid` _linkeddoor
                (:`Is Valid`
                  (`/Game/Blueprints/BP_DoorRotating.OnUnlocking` _linkeddoor)
                  (`ActorComponent.K2_DestroyComponent` (`self.Box`)))
                (:`Is Not Valid`
                  (`KismetSystemLibrary.PrintString` "SpellLock does not have a linked door!" true true (struct :`R` 1.0 :`G` 0.004727 :`A` 1.0) 10.0)))))))
      (:`CastFailed`
        (bind _assummoned_spell_damage_companion (cast `SummonedSpellDamageCompanion` OtherActor)
          (:`then`
            (set `self.CastIndex` 1))
          (:`CastFailed`
            (bind _asbp_fire_shotgun (cast `/Game/Blueprints/Combat/BP_FireShotgun` OtherActor))
            (set `self.CastIndex` 2)
            (goto _label)))))))

(fn `ActivateCrystal`
  (set `self.isActivated` true)
  (`NiagaraFunctionLibrary.SpawnSystemAtLocation` (`self.UnlockEffect`) (`SceneComponent.K2_GetComponentLocation` (`self.StaticMesh`))))

(fn `UserConstructionScript`
  (bind _unlockedeffect (`self.UnlockedEffect`))
  (switch `int` (`self.RequiredIDToUnlockDoor`)
    (:`1`
      ;[0 0 0] Shield break effect
      (set `self.UnlockEffect` "/Game/MagicalProjectile/FX/Impact/NS_IMpact_06.NS_IMpact_06")
      ;[0 0 0] Shield effect
      (`NiagaraComponent.SetAsset` _unlockedeffect "/Game/MagicalProjectile/FX/Projectile/NS_ProjE_00.NS_ProjE_00" true))
    (:`2`
      (set `self.UnlockEffect` "/Game/MagicalProjectile/FX/Impact/NS_IMpact_09.NS_IMpact_09")
      (`NiagaraComponent.SetAsset` _unlockedeffect "/Game/MagicalProjectile/FX/Projectile/NS_ProjA_01.NS_ProjA_01" true))
    (:`3`
      (set `self.UnlockEffect` "/Game/MagicalProjectile/FX/Impact/NS_IMpact_00.NS_IMpact_00")
      (`NiagaraComponent.SetAsset` _unlockedeffect "/Game/MagicalProjectile/FX/Projectile/NS_ProjB_04.NS_ProjB_04" true))
    (:`4`
      (set `self.UnlockEffect` "/Game/MagicalProjectile/FX/Impact/NS_IMpact_03.NS_IMpact_03")
      (`NiagaraComponent.SetAsset` _unlockedeffect "/Game/MagicalProjectile/FX/Projectile/NS_ProjA_01.NS_ProjA_01" true))
    (:`5`
      (set `self.UnlockEffect` "/Game/MagicalProjectile/FX/Impact/NS_IMpact_01.NS_IMpact_01")
      (`NiagaraComponent.SetAsset` _unlockedeffect "/Game/MegaMagicVFXBundle/VFX/MagicShieldsVFX/VFX/DefaultVersions/WindShield/Systems/N_WindShield.N_WindShield" true))))