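; BP_DoorRotating is a stone door that rotates its Cube toward -90 yaw on the second unlock call, with Wwise audio.
; A timeline feeds its alpha as DeltaTime into RInterpToConstant; closing reverses that timeline, keeping the same target.
; After a short BeginPlay delay it restores state from JamGameInstanceSubsystem save data.
; On load, an unlocked door gets its relative location set to TargetHeight, not its rotation.
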(event `self.ReceiveBeginPlay`
  (`KismetSystemLibrary.Delay` 0.2)
  (bind _returnvalue (message `SaveGameInterface.GetSaveGameData` (subsystem `JamGameInstanceSubsystem`)))
  (`/Engine/EditorBlueprintResources/StandardMacros.IsValid` _returnvalue
    (:`Is Valid`
      (`self.SetStateFromSaveData` (`JamSaveGameObject.WorldData` _returnvalue))
      (`self.OnWorldLoad`))))

(event `OnUnlocking`
  (bind _cube (`self.Cube`))
  (if (`self.FirstSpell?`)
    (set `self.isUnlocked` true)
    (`AkGameplayStatics.PostEvent` "/Game/WwiseAudio/StoneDoorOpen.StoneDoorOpen" self)
    (bind (_direction _alpha) (`Timeline|Timeline_0` :!label _label)
      (:`Update`
        (`SceneComponent.K2_SetRelativeRotation` _cube (`KismetMathLibrary.RInterpTo_Constant` (`SceneComponent.RelativeRotation` _cube) (struct :`Yaw` -90.0) _alpha (`self.RotationSpeed`)) false false)))
    (else
      (set `self.FirstSpell?` true))))

(event `OnClose`
  (if (`self.isUnlocked`)
    (`|ExecutionSequence`
      (:`then_0`
        (set `self.isUnlocked` false)
        (`AkGameplayStatics.PostEvent` "/Game/WwiseAudio/StoneDoorOpen.StoneDoorOpen" self))
      (:`then_1`
        (goto _label :!via `ReverseFromEnd`)))))

(event `OnWorldLoad`
  (if (`self.isUnlocked`)
    (`SceneComponent.K2_SetRelativeLocation` (`self.Cube`) (`KismetMathLibrary.MakeVector` 0.0 0.0 (`self.TargetHeight`)) false false)))

(fn `UserConstructionScript`)