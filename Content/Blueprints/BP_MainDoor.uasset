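; Main stone door that unlocks once the player carries both the red and black potions.
; Potion check triggers light the matching potion glass and attempt the unlock, which raises a spotlight and illuminates the door relief; BeginPlay restores this from the player's flags.
; When unlocked, the trigger box slides the door with a timeline and Wwise sound, reversing on exit.
; Otherwise it plays HUD animations showing which potion is missing.
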(event `self.ReceiveBeginPlay`
  (bind _playerref (`self.PlayerRef`))
  (bind _asbp_jam_player_character (cast `/Game/Player/BP_JamPlayerCharacter` (`GameplayStatics.GetPlayerCharacter` 0)))
  (set `self.PlayerRef` _asbp_jam_player_character)
  (set `self.Player State Ref` (`/Game/Blueprints/BFL_CommonFunctions.GetPlayerStateRef`))
  (`KismetSystemLibrary.Delay` 2.0)
  (if (and (`JamPlayerCharacter.hasRedPotion` _playerref) (`JamPlayerCharacter.hasBlackPotion` _playerref))
    (`self.UnlockDoor`)
    (elif (and (`JamPlayerCharacter.hasBlackPotion` (`self.PlayerRef`)) (not (`JamPlayerCharacter.hasRedPotion` (`self.PlayerRef`))))
      (`PrimitiveComponent.SetMaterial` (`self.BlackPotion`) 2 "/Game/Fab/Potion/MI_WhiteGlass.MI_WhiteGlass")
      (`KismetSystemLibrary.Delay` 0.2)
      (`ActorComponent.K2_DestroyComponent` (`self.BlackPotionCheck`))
      (elif (and (not (`JamPlayerCharacter.hasBlackPotion` (`self.PlayerRef`))) (`JamPlayerCharacter.hasRedPotion` (`self.PlayerRef`)))
        (`PrimitiveComponent.SetMaterial` (`self.RedPotion`) 2 "/Game/Fab/Potion/MI_WhiteGlass.MI_WhiteGlass")
        (`KismetSystemLibrary.Delay` 0.2)
        (`ActorComponent.K2_DestroyComponent` (`self.RedPotionCheck`))))))

(event `UnlockDoor`
  (bind _playerref (`self.PlayerRef`))
  (if (and (`JamPlayerCharacter.hasRedPotion` _playerref) (`JamPlayerCharacter.hasBlackPotion` _playerref))
    (set `self.isUnlocked` true)
    (`LightComponent.SetIntensity` (`self.SpotLight`) 16.0)
    (`PrimitiveComponent.SetMaterial` (`self.DoorRelief`) 1 "/Game/Fab/Potion/MI_BlackGlassIlluminated.MI_BlackGlassIlluminated")))

(event `OpenDoor`
  (`AkGameplayStatics.PostEvent` "/Game/WwiseAudio/StoneDoorOpen.StoneDoorOpen" self)
  (bind (_direction _doorlocationvector) (`Timeline|OpenDoorTL` :!label _label)
    (:`Update`
      (`SceneComponent.K2_SetRelativeLocation` (`self.MainDoor`) (* _doorlocationvector (`KismetMathLibrary.MakeVector` 0.0 0.0 (* (`self.DoorHeight`) -1.0))) false false))))

(event `CloseDoor`
  (`AkGameplayStatics.PostEvent` "/Game/WwiseAudio/StoneDoorOpen.StoneDoorOpen" self)
  (goto _label :!via `ReverseFromEnd`))

(event `self.OpenCloseTriggerBox.OnComponentBeginOverlap`
  (params (OverlappedComponent :type "PrimitiveComponent Object Reference") (OtherActor :type "Actor Object Reference") (OtherComp :type "PrimitiveComponent Object Reference") (OtherBodyIndex :type Integer) (bFromSweep :type Boolean) (SweepResult :type "HitResult Structure (by ref)"))
  (if (and (== OtherActor (`self.PlayerRef`)) (`self.isUnlocked`))
    (`self.OpenDoor`)
    (else
      (`/Engine/EditorBlueprintResources/StandardMacros.DoOnce` false :!label _label_2
        (:`Completed`
          (`self.DisplayNeededPotion`))))))

(event `self.OpenCloseTriggerBox.OnComponentEndOverlap`
  (params (OverlappedComponent :type "PrimitiveComponent Object Reference") (OtherActor :type "Actor Object Reference") (OtherComp :type "PrimitiveComponent Object Reference") (OtherBodyIndex :type Integer))
  (if (and (== OtherActor (`self.PlayerRef`)) (`self.isUnlocked`))
    (`self.CloseDoor`)
    (goto _label_2 :!via `Reset`)
    (else
      (goto _label_2 :!via `Reset`))))

(event `self.BlackPotionCheck.OnComponentBeginOverlap`
  (params (OverlappedComponent :type "PrimitiveComponent Object Reference") (OtherActor :type "Actor Object Reference") (OtherComp :type "PrimitiveComponent Object Reference") (OtherBodyIndex :type Integer) (bFromSweep :type Boolean) (SweepResult :type "HitResult Structure (by ref)"))
  (bind _playerref (`self.PlayerRef`))
  (if (and (== OtherActor _playerref) (`JamPlayerCharacter.hasBlackPotion` _playerref))
    (`PrimitiveComponent.SetMaterial` (`self.BlackPotion`) 2 "/Game/Fab/Potion/MI_WhiteGlass.MI_WhiteGlass")
    (`self.UnlockDoor`)
    (`KismetSystemLibrary.Delay` 0.2)
    (`ActorComponent.K2_DestroyComponent` (`self.BlackPotionCheck`))))

(event `self.RedPotionCheck.OnComponentBeginOverlap`
  (params (OverlappedComponent :type "PrimitiveComponent Object Reference") (OtherActor :type "Actor Object Reference") (OtherComp :type "PrimitiveComponent Object Reference") (OtherBodyIndex :type Integer) (bFromSweep :type Boolean) (SweepResult :type "HitResult Structure (by ref)"))
  (bind _playerref (`self.PlayerRef`))
  (if (and (== OtherActor _playerref) (`JamPlayerCharacter.hasRedPotion` _playerref))
    (`/Engine/EditorBlueprintResources/StandardMacros.IncrementInt` (`self.PotionsCollected`)
      (:`  `
        (`PrimitiveComponent.SetMaterial` (`self.RedPotion`) 2 "/Game/Fab/Potion/MI_WhiteGlass.MI_WhiteGlass")
        (`self.UnlockDoor`)
        (`KismetSystemLibrary.Delay` 0.2)
        (`ActorComponent.K2_DestroyComponent` (`self.RedPotionCheck`))))))

(fn `DisplayNeededPotion`
  (bind _hudref (`/Game/Player/BP_JamPlayerState.HUDRef` (`self.Player State Ref`)))
  (bind _hudref_2 (`/Game/Player/BP_JamPlayerState.HUDRef` (`self.Player State Ref`)))
  (bind _hudref_3 (`/Game/Player/BP_JamPlayerState.HUDRef` (`self.Player State Ref`)))
  (bind _hudref_4 (`/Game/Player/BP_JamPlayerState.HUDRef` (`self.Player State Ref`)))
  (if (and (`JamPlayerCharacter.hasBlackPotion` (`self.PlayerRef`)) (not (`JamPlayerCharacter.hasRedPotion` (`self.PlayerRef`))))
    (`UserWidget.PlayAnimation` _hudref_2 (`/Game/UI/Common/Widgets/HUD/WB_MainHUD.NeedRedPotion` _hudref_2) 0.0 1 "Forward" 1.0 false)
    (elif (and (not (`JamPlayerCharacter.hasBlackPotion` (`self.PlayerRef`))) (`JamPlayerCharacter.hasRedPotion` (`self.PlayerRef`)))
      (`UserWidget.PlayAnimation` _hudref_3 (`/Game/UI/Common/Widgets/HUD/WB_MainHUD.NeedBlackPotion` _hudref_3) 0.0 1 "Forward" 1.0 false)
      (elif (and (not (`JamPlayerCharacter.hasBlackPotion` (`self.PlayerRef`))) (not (`JamPlayerCharacter.hasRedPotion` (`self.PlayerRef`))))
        (`UserWidget.PlayAnimation` _hudref (`/Game/UI/Common/Widgets/HUD/WB_MainHUD.NeedRedPotion` _hudref) 0.0 1 "Forward" 1.0 false)
        (`UserWidget.PlayAnimation` _hudref_4 (`/Game/UI/Common/Widgets/HUD/WB_MainHUD.NeedBlackPotion` _hudref_4) 0.0 1 "Forward" 1.0 false)))))

(fn `UserConstructionScript`)