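; BP_TranslatableGlyph is a glyph actor that reveals its translated text when the player interacts with it.
; Interacting, if allowed, waits briefly, flags it translated, unhides the TextRender and resets the actor's tags.
; On BeginPlay it restores state from the game instance subsystem's save data, replaying the reveal if already translated.
; The construction script applies the per-instance material and text, and resets tags on non-interactable glyphs.
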(event `self.ReceiveBeginPlay`
  (bind _returnvalue (message `SaveGameInterface.GetSaveGameData` (subsystem `JamGameInstanceSubsystem`)))
  (`/Engine/EditorBlueprintResources/StandardMacros.IsValid` _returnvalue
    (:`Is Valid`
      (`self.SetStateFromSaveData` (`JamSaveGameObject.WorldData` _returnvalue))
      (if (`self.isTranslated`)
        (`self.OnWorldLoad`)))))

(event `InteractInterface.Interact`
  (if (`self.isInteractable?`)
    (`KismetSystemLibrary.Delay` 0.2)
    (set `self.isTranslated` true)
    (`SceneComponent.SetHiddenInGame` (`self.TextRender`) false false :!label _label)
    (set `self.Tags` (`|MakeArray` "None" :!type "Name"))))

(event `OnWorldLoad`
  (goto _label))

(fn `UserConstructionScript`
  (`PrimitiveComponent.SetMaterial` (`self.StaticMesh`) 0 (`self.MaterialInstance`))
  (`TextRenderComponent.K2_SetText` (`self.TextRender`) (`self.TranslatedText`))
  (if (not (`self.isInteractable?`))
    (set `self.Tags` (`|MakeArray` "None" :!type "Name"))))