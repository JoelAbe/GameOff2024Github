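; Glyph pedestal that unlocks spells when the player presses a correct three-button glyph combination.
; BP_GlyphButtons report values to it, and the third press checks the ordered combo against a data table, briefly locking all buttons.
; A match adds and equips the spell with HUD, audio and Niagara feedback, unless already owned.
; Pressed buttons then show the result overlay and reset, as they do after an inactivity timeout.
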(event `self.ReceiveBeginPlay`
  (set `self.Player Character Ref` (`/Game/Blueprints/BFL_CommonFunctions.GetPlayerCharacterRef`))
  (set `self.Player State Ref` (`/Game/Blueprints/BFL_CommonFunctions.GetPlayerStateRef`))
  (bind _outactors (`GameplayStatics.GetAllActorsOfClass` "/Game/Blueprints/GlyphItems/BP_GlyphButton.BP_GlyphButton_C"))
  (set `self.GlyphButtons` _outactors))

(event `ReceiveButtonValue`
  (params (ButtonValue :type Integer) (ButtonReference :type "/Game/Blueprints/GlyphItems/BP_GlyphButton Object Reference"))
  (bind _returnvalue (`KismetArrayLibrary.Array_Add` (`self.PressedCombo`) ButtonValue))
  (bind _returnvalue_2 (`KismetArrayLibrary.Array_Add` (`self.PressedButtons`) ButtonReference))
  ;[1 1 1] Timer for inactivity
  (`KismetSystemLibrary.K2_ClearTimer` null "ClearAndLightButtons")
  (`KismetSystemLibrary.K2_SetTimer` null "ClearAndLightButtons" 5.0)
  (if (== _returnvalue 2)
    (`self.CheckGlyphCombination`)
    (for _array_element (`self.GlyphButtons`)
      (set `/Game/Blueprints/GlyphItems/BP_GlyphButton.AllowButtonPress` false _array_element))
    (`KismetSystemLibrary.Delay` 0.5)
    (if (and (`self.ComboCorrect`) (not (`self.PlayerHasSpell`)))
      (`ActorComponent.Activate` (`self.Niagara`) false)
      (`AkGameplayStatics.PostEvent` "/Game/WwiseAudio/VortexImpact.VortexImpact" (`self.Player Character Ref`))
      (`ActorComponent.Activate` (`/Game/Player/BP_JamPlayerCharacter.N_MagicalBarrier` (`self.Player Character Ref`)) false))
    (`self.ClearAndLightButtons`)
    (`KismetSystemLibrary.Delay` 1.5)
    (for _array_element_2 (`self.GlyphButtons`)
      (set `/Game/Blueprints/GlyphItems/BP_GlyphButton.AllowButtonPress` true _array_element_2))
    (set `self.PlayerHasSpell` false)
    (`ActorComponent.Deactivate` (`/Game/Player/BP_JamPlayerCharacter.N_MagicalBarrier` (`self.Player Character Ref`)))))

(fn `AddSpellToPlayer`
  (params (SpellIDToAdd :type Integer))
  (bind _hudref (`/Game/Player/BP_JamPlayerState.HUDRef` (`self.Player State Ref`)))
  ;[0.05 0.05 0.05] Pick spell by ID here
  (bind _returnvalue (`|GetDataTableRow` "/Game/Game/Data/DT_Spells.DT_Spells" (`KismetStringLibrary.Conv_StringToName` (`KismetStringLibrary.Conv_IntToString` SpellIDToAdd)))
    (:`then`
      ;[0 0 0] If the player has the spell, break and tell them they've already unlocked it. Otherwise, add it
      (for _array_element (`InventoryComponent.Inventory` (`JamPlayerCharacter.InventoryComponent` (`self.Player Character Ref`)))
        (if (== (`.ID` (break `Spell` _array_element)) (`.ID` (break `Spell` _returnvalue)))
          (set `self.PlayerHasSpell` true)
          (break)))
      (if (`self.PlayerHasSpell`)
        (`KismetSystemLibrary.PrintString` "You've already unlocked that spell!")
        (else
          (`InventoryComponent.Add` (`JamPlayerCharacter.InventoryComponent` (`self.Player Character Ref`)) _returnvalue)
          (`/Game/Player/BP_JamPlayerState.SetEquippedSpell` (`self.Player State Ref`) _returnvalue)
          (set `self.PlayerHasSpell` false)
          (`AkGameObject.PostAkEvent` :`self` (`/Game/Player/BP_JamPlayerCharacter.AK_SpellCast` (`self.Player Character Ref`)) :`AkEvent` "/Game/WwiseAudio/SpellLearned.SpellLearned")
          (`UserWidget.PlayAnimation` _hudref (`/Game/UI/Common/Widgets/HUD/WB_MainHUD.UnlockedSpell` _hudref) 0.0 1 "Forward" 1.0 false))))))

(fn `CheckGlyphCombination`
  (bind _outrownames (`DataTableFunctionLibrary.GetDataTableRowNames` "/Game/Game/Data/DT_GlyphCombinationsTable.DT_GlyphCombinationsTable"))
  (for _array_element _outrownames
    (bind _returnvalue (`|GetDataTableRow` "/Game/Game/Data/DT_GlyphCombinationsTable.DT_GlyphCombinationsTable" _array_element)
      (:`then`
        (bind (_id _unlockedid _glyphcombination) (break `/Game/Game/Data/S_GlyphCombinations` _returnvalue))
        (bind _returnvalue_2 (`KismetArrayLibrary.Array_Identical` _glyphcombination (`self.PressedCombo`)))
        (if _returnvalue_2
          (`self.AddSpellToPlayer` _id)
          (set `self.ComboCorrect` _returnvalue_2))))))

(fn `ClearAndLightButtons`
  (bind _pressedbuttons (`self.PressedButtons`))
  (`KismetArrayLibrary.Array_Clear` (`self.PressedCombo`))
  (for _array_element _pressedbuttons
    (bind _asbp_glyph_button (cast `/Game/Blueprints/GlyphItems/BP_GlyphButton` _array_element))
    (`/Game/Blueprints/GlyphItems/BP_GlyphButton.SetGlyphOverlay` _asbp_glyph_button (`self.ComboCorrect`)))
  (`KismetArrayLibrary.Array_Clear` _pressedbuttons)
  (set `self.ComboCorrect` false)
  (`KismetSystemLibrary.PrintString` "Set False"))

(fn `UserConstructionScript`)