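; A pressable glyph button for a pedestal puzzle, showing a glyph material set in the construction script.
; Interact, when allowed, plays a Wwise sound, animates the mesh in and back out with timelines that block re-pressing, and sends its number and self to the BP_GlyphPedestal found at BeginPlay.
; SetGlyphOverlay briefly tints the button with one of two overlay materials for correct or incorrect feedback, then clears it.
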(event `self.ReceiveBeginPlay`
  (bind _returnvalue (`GameplayStatics.GetActorOfClass` "/Game/Blueprints/GlyphItems/BP_GlyphPedestal.BP_GlyphPedestal_C")))

(event `InteractInterface.Interact`
  (if (`self.AllowButtonPress`)
    (`self.ButtonClicked`)
    (`/Game/Blueprints/GlyphItems/BP_GlyphPedestal.ReceiveButtonValue` (stale `self.ReceiveBeginPlay` _returnvalue) (`self.GetButtonNumber`) self)))

(event `ButtonClicked`
  ;[1 1 1] Button Clicked
  (`AkGameplayStatics.PostEvent` "/Game/WwiseAudio/PedButtons.PedButtons" self)
  (set `self.AllowButtonPress` false)
  (bind (_direction _buttonvector) (`Timeline|ButtonClickedTimeline` :!via `PlayFromStart`)
    (:`Update`
      (`SceneComponent.K2_SetRelativeLocation` (`self.StaticMesh`) _buttonvector false false))
    (:`Finished`
      (bind (_direction_2 _buttonvector_2) (`Timeline|Timeline` :!via `ReverseFromEnd`)
        (:`Update`
          (`SceneComponent.K2_SetRelativeLocation` (`self.StaticMesh`) _buttonvector_2 false false))
        (:`Finished`
          (set `self.AllowButtonPress` true))))))

(event `SetGlyphOverlay`
  (params (isCorrect :type Boolean))
  (bind _staticmesh (`self.StaticMesh`))
  (if isCorrect
    (`MeshComponent.SetOverlayMaterial` _staticmesh "/Engine/ArtTools/RenderToTexture/Materials/M_RadiusDebugTranslucent.M_RadiusDebugTransLucent")
    (else
      (`MeshComponent.SetOverlayMaterial` _staticmesh "/Engine/EngineDebugMaterials/M_SimpleTranslucent.M_SimpleTranslucent")))
  (`KismetSystemLibrary.Delay` 2.0)
  (`MeshComponent.SetOverlayMaterial` (`self.StaticMesh`) null))

(fn `UserConstructionScript`
  (`PrimitiveComponent.SetMaterial` (`self.GlyphPainting`) 0 (`self.Material`)))