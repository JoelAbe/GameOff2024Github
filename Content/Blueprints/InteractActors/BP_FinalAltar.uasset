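; BP_FinalAltar is an interactable altar that triggers the game's ending based on the potions the player carries.
; It caches the jam player character on BeginPlay and responds to Interact only after the final boss is beaten.
; Red and black potions are required, and adding white selects the good ending over the bad one.
; Each outcome activates fire effects and reveals the placed potion meshes before calling its ending dispatcher.
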(event `self.ReceiveBeginPlay`
  (`parent.ReceiveBeginPlay`)
  (bind _asbp_jam_player_character (cast `/Game/Player/BP_JamPlayerCharacter` (`GameplayStatics.GetPlayerCharacter` 0)))
  (set `self.PlayerRef` _asbp_jam_player_character))

(event `InteractInterface.Interact`
  (bind _playerref (`self.PlayerRef`))
  (bind _playerref_2 (`self.PlayerRef`))
  (if (`/Game/Player/BP_JamPlayerCharacter.beatFinalBoss?` _playerref_2)
    (if (and (`JamPlayerCharacter.hasRedPotion` _playerref_2) (`JamPlayerCharacter.hasBlackPotion` _playerref_2))
      (if (and (`JamPlayerCharacter.hasRedPotion` _playerref) (`JamPlayerCharacter.hasBlackPotion` _playerref) (`JamPlayerCharacter.hasWhitePotion` _playerref))
        (`ActorComponent.Activate` (`self.Fire`) false)
        (`ActorComponent.Activate` (`self.Fire2`) false)
        (`ActorComponent.Activate` (`self.Fire1`) false)
        (`SceneComponent.SetVisibility` (`self.BlackPotionMesh`) true false)
        (`SceneComponent.SetVisibility` (`self.WhitePotionMesh`) true false)
        (`SceneComponent.SetVisibility` (`self.RedPotionMesh`) true false)
        (`self.OnGoodEnding`)
        (else
          (`ActorComponent.Activate` (`self.Fire1`) false)
          (`ActorComponent.Activate` (`self.Fire2`) false)
          (`SceneComponent.SetVisibility` (`self.BlackPotionMesh`) true false)
          (`SceneComponent.SetVisibility` (`self.RedPotionMesh`) true false)
          (`self.OnBadEnding`)))
      (else
        (`KismetSystemLibrary.PrintString` "Missing Potions")))))

(fn `UserConstructionScript`
  (`parent.UserConstructionScript`))