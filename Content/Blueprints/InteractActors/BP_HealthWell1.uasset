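; BP_HealthWell1 is an interactable health well that heals the player character.
; It caches a player character reference on BeginPlay.
; On Interact, if Health is below MaxHealth, it adds a fixed amount of health through the player's Attributes and plays a 2D drinking sound with slightly randomized pitch.
; The graph sets no cooldown or use limit, so it works whenever the player is below full health.
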(event `self.ReceiveBeginPlay`
  (set `self.Player Character Ref` (`/Game/Blueprints/BFL_CommonFunctions.GetPlayerCharacterRef`)))

(event `InteractInterface.Interact`
  (bind _attributes (`JamPlayerCharacter.Attributes` (`self.Player Character Ref`)))
  (if (< (`AttributesComponent.Health` _attributes) (`AttributesComponent.MaxHealth` _attributes))
    (`AttributesComponent.AddHealth` (`JamPlayerCharacter.Attributes` (`self.Player Character Ref`)) 100.0)
    (`GameplayStatics.PlaySound2D` "/Game/NonWwiseSounds/574077__valentinpetiteau__potion-drink-swallow.574077__valentinpetiteau__potion-drink-swallow" 1.0 (`KismetMathLibrary.RandomFloatInRange` 0.9 1.1) 0.0 null null false)))

(fn `UserConstructionScript`)