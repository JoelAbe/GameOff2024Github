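; BP_BlackPotion is an interactable black potion pickup that bobs up and down each Tick using a sine of game time.
; On BeginPlay it caches the player character and, after a one-second delay, destroys itself if the player already has the potion.
; Interact sets HasBlackPotion on the player, makes the HUD's BlackPotion element opaque through the player state's HUD reference, then destroys the actor.
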(event `self.ReceiveBeginPlay`
  (bind _playerref (`self.PlayerRef`))
  (bind _asbp_jam_player_character (cast `/Game/Player/BP_JamPlayerCharacter` (`GameplayStatics.GetPlayerCharacter` 0)))
  (set `self.PlayerRef` _asbp_jam_player_character)
  (`KismetSystemLibrary.Delay` 1.0)
  (`/Engine/EditorBlueprintResources/StandardMacros.IsValid` _playerref
    (:`Is Valid`
      (if (`JamPlayerCharacter.hasBlackPotion` _playerref)
        (`self.K2_DestroyActor`)))))

(event `InteractInterface.Interact`
  (bind _playerref (`self.PlayerRef`))
  (set `JamPlayerCharacter.hasBlackPotion` true _playerref)
  (`Widget.SetRenderOpacity` (`/Game/UI/Common/Widgets/HUD/WB_MainHUD.BlackPotion` (`/Game/Player/BP_JamPlayerState.HUDRef` (`/Game/Player/BP_JamPlayerCharacter.BP Player State Ref` _playerref))) 1.0)
  (`self.K2_DestroyActor`))

(event `self.ReceiveTick`
  (params (DeltaSeconds :type "Float (single-precision)"))
  (`SceneComponent.K2_AddRelativeLocation` (`self.StaticMesh`) (`KismetMathLibrary.MakeVector` 0.0 0.0 (* (`KismetMathLibrary.Sin` (`self.GetGameTimeSinceCreation`)) 0.1)) false false))

(fn `UserConstructionScript`)