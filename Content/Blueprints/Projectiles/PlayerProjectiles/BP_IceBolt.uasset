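; Ice bolt player projectile that slows the NPC it hits for two seconds.
; It plays Wwise cast and impact sounds at its location on spawn and hit.
; On a valid hit it switches off its particle and waits out the delay before destroying itself, ending the slow on NPC characters first.
; With no valid hit actor, it flags itself to destroy on hit instead.
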(event `self.ReceiveBeginPlay`
  (`AkGameplayStatics.PostEventAtLocation` "/Game/WwiseAudio/IceCast.IceCast" (`self.K2_GetActorLocation`) (`KismetMathLibrary.Conv_VectorToRotator` (`self.GetActorForwardVector`))))

(event `self.OnProjectileHit`
  (`AkGameplayStatics.PostEventAtLocation` "/Game/WwiseAudio/IceImpact.IceImpact" (`self.K2_GetActorLocation`) (`KismetMathLibrary.Conv_VectorToRotator` (`self.GetActorForwardVector`)))
  (if (`KismetSystemLibrary.IsValid` (`self.HitActor`))
    (bind _asnpcbase_character (cast `NPCBaseCharacter` (`self.HitActor`))
      (:`then`
        (`NPCBaseCharacter.StartSlow` _asnpcbase_character)
        (`ActorComponent.Deactivate` (`self.ProjectileParticle`))
        (`KismetSystemLibrary.Delay` 2.0)
        (`NPCBaseCharacter.EndSlow` _asnpcbase_character)
        (`self.K2_DestroyActor`))
      (:`CastFailed`
        (`ActorComponent.Deactivate` (`self.ProjectileParticle`))
        (`KismetSystemLibrary.Delay` 2.0)
        (`self.K2_DestroyActor`)))
    (else
      (set `self.DestroyOnHit` true))))

(fn `UserConstructionScript`)