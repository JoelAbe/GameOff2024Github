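; Player gravity ball projectile that stops after a short flight and pulls nearby NPCs toward itself.
; On stopping, it takes a one-time snapshot of NPC characters overlapping its sphere.
; For a few seconds, Tick uses swept, interpolated moves to draw them in, skipping dead or super-armored ones, and prints their names.
; It plays a Wwise cast sound on spawn, and deactivates its particle before destroying itself.
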(event `self.ReceiveBeginPlay`
  (`AkGameplayStatics.PostEventAtLocation` "/Game/WwiseAudio/GravCast.GravCast" (`self.K2_GetActorLocation`) (`KismetMathLibrary.Conv_VectorToRotator` (`self.GetActorForwardVector`)))
  (`KismetSystemLibrary.Delay` 1.0)
  (`MovementComponent.StopMovementImmediately` (`self.ProjectileMovementComponent`))
  (for _array_element (`PrimitiveComponent.GetOverlappingActors` (`self.Sphere`) "/Script/CommonUI_FPSBase.NPCBaseCharacter")
    (bind _asnpcbase_character (cast `NPCBaseCharacter` _array_element))
    (bind _output_get (set `self.As NPCBase Character` _asnpcbase_character))
    (`KismetArrayLibrary.Array_AddUnique` (`self.NPCsToPull`) _output_get))
  (set `self.ReadyToPull` true)
  (`KismetSystemLibrary.Delay` 3.0)
  (`ActorComponent.Deactivate` (`self.ProjectileParticle`))
  (set `self.ReadyToPull` false)
  (`KismetSystemLibrary.Delay` 1.0)
  (`self.K2_DestroyActor`))

(event `self.ReceiveTick`
  (params (DeltaSeconds :type "Float (single-precision)"))
  (if (`self.ReadyToPull`)
    (for _array_element (`self.NPCsToPull`)
      (if (and (not (`NPCBaseCharacter.isDead` _array_element)) (not (`NPCBaseCharacter.hasSuperArmor` _array_element)))
        (`self.K2_SetActorLocation` _array_element (`KismetMathLibrary.VInterpTo` (`self.K2_GetActorLocation` _array_element) (`self.K2_GetActorLocation`) DeltaSeconds 10.0) true false)))
    (for _array_element_2 (`self.NPCsToPull`)
      (`KismetSystemLibrary.PrintString` (`KismetSystemLibrary.GetDisplayName` _array_element_2)))))

(fn `UserConstructionScript`)