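; BP_ArcaneBlast is an arcane blast projectile Blueprint, filed under player projectiles, with its own audio and owner-dependent setup.
; Wwise events play the cast sound on launch and the impact sound on hit, at the projectile's location and facing.
; On BeginPlay, when the owner is not the player character, it switches the mesh to a custom collision object type and overrides the movement component's initial and maximum speed.
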(event `self.OnLaunch`
  (`AkGameplayStatics.PostEventAtLocation` "/Game/WwiseAudio/ArcaneCast.ArcaneCast" (`self.K2_GetActorLocation`) (`KismetMathLibrary.Conv_VectorToRotator` (`self.GetActorForwardVector`))))

(event `self.ReceiveBeginPlay`
  (bind _projectilemovementcomponent (`self.ProjectileMovementComponent`))
  (if (!= (`self.GetOwner`) (`GameplayStatics.GetPlayerCharacter` 0))
    (`PrimitiveComponent.SetCollisionObjectType` (`self.ProjectileMesh`) "ECC_GameTraceChannel2")
    (set `ProjectileMovementComponent.InitialSpeed` 3500.0 _projectilemovementcomponent)
    (set `ProjectileMovementComponent.MaxSpeed` 3500.0 _projectilemovementcomponent)))

(event `self.OnProjectileHit`
  (`AkGameplayStatics.PostEventAtLocation` "/Game/WwiseAudio/ArcaneImpact.ArcaneImpact" (`self.K2_GetActorLocation`) (`KismetMathLibrary.Conv_VectorToRotator` (`self.GetActorForwardVector`))))

(fn `UserConstructionScript`)