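; BP_Door is a lockable sliding door that opens for the player and restores its state from save data.
; Lock and unlock events set IsUnlocked and swap two door mesh materials.
; When unlocked, trigger overlaps by the player drive a timeline that moves the mesh vertically toward TargetHeight or back, with a Wwise sound.
; After a delayed BeginPlay, it loads saved world data and reapplies the open material if unlocked.
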(event `self.ReceiveBeginPlay`
  (`KismetSystemLibrary.Delay` 2.0)
  (bind _returnvalue (message `SaveGameInterface.GetSaveGameData` (subsystem `JamGameInstanceSubsystem`)))
  (`/Engine/EditorBlueprintResources/StandardMacros.IsValid` _returnvalue
    (:`Is Valid`
      (`self.SetStateFromSaveData` (`JamSaveGameObject.WorldData` _returnvalue))
      (`self.OnWorldLoad`))
    (:`Is Not Valid`
      (`KismetSystemLibrary.PrintString` "Save data not valid - door"))))

(event `OnLock`
  (set `self.isUnlocked` false)
  (`PrimitiveComponent.SetMaterial` (`self.DoorMesh`) 5 "/Game/Fab/Potion/MI_LockedDoor.MI_LockedDoor")
  (`PrimitiveComponent.SetMaterial` (`self.DoorMesh`) 6 "/Game/Fab/Potion/MI_LockedDoor.MI_LockedDoor"))

(event `OnUnlocking`
  (set `self.isUnlocked` true)
  (`PrimitiveComponent.SetMaterial` (`self.DoorMesh`) 5 "/Game/Fab/Potion/MI_OpenDoor.MI_OpenDoor" :!label _label)
  (`PrimitiveComponent.SetMaterial` (`self.DoorMesh`) 6 "/Game/Fab/Potion/MI_OpenDoor.MI_OpenDoor"))

(event `OnWorldLoad`
  (if (`self.isUnlocked`)
    (goto _label)))

(event `OnOpen`
  (`AkGameplayStatics.PostEvent` "/Game/WwiseAudio/StoneDoorOpen.StoneDoorOpen" self)
  (set `self.isOpen` true)
  (bind (_direction _elevatorlocation) (`Timeline|Timeline_0` :!label _label_2)
    (:`Update`
      (`SceneComponent.K2_SetRelativeLocation` (`self.DoorMesh`) (* _elevatorlocation (`KismetMathLibrary.MakeVector` 0.0 0.0 (`self.TargetHeight`))) false false))))

(event `OnClose`
  (if (`self.isUnlocked`)
    (`AkGameplayStatics.PostEvent` "/Game/WwiseAudio/StoneDoorOpen.StoneDoorOpen" self)
    (set `self.isOpen` false)
    (goto _label_2 :!via `ReverseFromEnd`)))

(event `self.DoorOpenTrigger.OnComponentBeginOverlap`
  (params (OverlappedComponent :type "PrimitiveComponent Object Reference") (OtherActor :type "Actor Object Reference") (OtherComp :type "PrimitiveComponent Object Reference") (OtherBodyIndex :type Integer) (bFromSweep :type Boolean) (SweepResult :type "HitResult Structure (by ref)"))
  (if (and (== OtherActor (`/Game/Blueprints/BFL_CommonFunctions.GetPlayerCharacterRef`)) (`self.isUnlocked`) (not (`self.isOpen`)))
    (`self.OnOpen`)))

(event `self.DoorOpenTrigger.OnComponentEndOverlap`
  (params (OverlappedComponent :type "PrimitiveComponent Object Reference") (OtherActor :type "Actor Object Reference") (OtherComp :type "PrimitiveComponent Object Reference") (OtherBodyIndex :type Integer))
  (if (and (== OtherActor (`/Game/Blueprints/BFL_CommonFunctions.GetPlayerCharacterRef`)) (`self.isUnlocked`))
    (`self.OnClose`)))

(fn `UserConstructionScript`)