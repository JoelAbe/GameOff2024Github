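; BP_AttributeItemPickup is a pickup that serves as either a health or mana item, chosen by the IsHealthPickup flag.
; The construction script uses that flag to set a heart or crystal mesh and the matching heal or arcane Niagara pickup effect.
; On pickup, it refreshes the player's health or mana widget through a cached character reference and posts the matching Wwise restore sound.
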(event `self.ReceiveBeginPlay`
  (set `self.Player Character Ref` (`/Game/Blueprints/BFL_CommonFunctions.GetPlayerCharacterRef`)))

(event `self.OnPickup`
  (bind _player_character_ref (`self.Player Character Ref`))
  (if (`self.isHealthPickup`)
    (`/Game/Player/BP_JamPlayerCharacter.SetHealthWidget` _player_character_ref)
    (`AkGameplayStatics.PostEvent` "/Game/WwiseAudio/RestoreHealth.RestoreHealth" self)
    (else
      (`/Game/Player/BP_JamPlayerCharacter.SetManaWidget` _player_character_ref)
      (`AkGameplayStatics.PostEvent` "/Game/WwiseAudio/RestoreMana.RestoreMana" self))))

(fn `UserConstructionScript`
  (if (`self.isHealthPickup`)
    (`StaticMeshComponent.SetStaticMesh` (`self.StaticMesh`) "/Game/CustomModels/heart.heart")
    (set `self.PickupEffect` "/Game/MagicAbilitiesVol2/Particles/NiagaraSystems/NS_BuffAoE09_Heal.NS_BuffAoE09_Heal")
    (else
      (`StaticMeshComponent.SetStaticMesh` (`self.StaticMesh`) "/Game/CustomModels/Crystal.Crystal")
      (set `self.PickupEffect` "/Game/MagicAbilitiesVol2/Particles/NiagaraSystems/NS_BuffAoE07_Arcane.NS_BuffAoE07_Arcane"))))