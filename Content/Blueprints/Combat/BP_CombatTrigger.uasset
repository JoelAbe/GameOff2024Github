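; Combat encounter trigger that seals doors and switches music to combat or boss-fight state when the player first enters its box.
; It notifies through triggered events, records each door's unlocked state, then closes and locks the open ones.
; On combat completion it restores those doors, unlocks any post-combat doors and sets victory music.
; Save data loaded shortly after BeginPlay keeps completed encounters from retriggering.
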(event `self.ReceiveBeginPlay`
  (`KismetSystemLibrary.Delay` 0.2)
  (bind _returnvalue (message `SaveGameInterface.GetSaveGameData` (subsystem `JamGameInstanceSubsystem`)))
  (`/Engine/EditorBlueprintResources/StandardMacros.IsValid` _returnvalue
    (:`Is Valid`
      (`self.SetStateFromSaveData` (`JamSaveGameObject.WorldData` _returnvalue))
      (if (`self.CombatComplete`)
        (set `self.CombatTriggered` true)))))

(event `OnCombatComplete`
  (set `self.CombatComplete` true)
  (`KismetSystemLibrary.PrintString` "Combat complete")
  (for (_array_element _array_index) (`self.DoorsState`)
    (if _array_element
      (`/Game/Blueprints/BP_Door.OnUnlocking` (`|GetArrayItem` (`self.DoorsArray`) _array_index))))
  ;[0 0 0] Stop music
  (`AkGameplayStatics.SetState` "/Game/WwiseAudio/SetStates/PlayerVictory.PlayerVictory")
  (for _array_element_2 (`self.DoorsToUnlockAfterCombat`)
    (`/Game/Blueprints/BP_Door.OnUnlocking` _array_element_2)))

(event `self.Box.OnComponentBeginOverlap`
  (params (OverlappedComponent :type "PrimitiveComponent Object Reference") (OtherActor :type "Actor Object Reference") (OtherComp :type "PrimitiveComponent Object Reference") (OtherBodyIndex :type Integer) (bFromSweep :type Boolean) (SweepResult :type "HitResult Structure (by ref)"))
  (if (and (== OtherActor (`GameplayStatics.GetPlayerCharacter` 0)) (not (`self.CombatTriggered`)))
    (set `self.CombatTriggered` true)
    (`self.OnCombatTriggered`)
    (for _array_element (`self.DoorsArray`)
      (`/Engine/EditorBlueprintResources/StandardMacros.IsValid` _array_element
        (:`Is Valid`
          (bind _isunlocked (`UnlockableDoor.isUnlocked` _array_element))
          (`KismetArrayLibrary.Array_Add` (`self.DoorsState`) _isunlocked)
          (if _isunlocked
            (`/Game/Blueprints/BP_Door.OnClose` _array_element)
            (`/Game/Blueprints/BP_Door.OnLock` _array_element)))))
    ;[0 0 0] Play music
    (if (`self.isBossFight`)
      (`AkGameplayStatics.SetState` "/Game/WwiseAudio/SetStates/BossCombat.BossCombat")
      (`self.OnBossCombatTriggered`)
      (else
        (`AkGameplayStatics.SetState` "/Game/WwiseAudio/SetStates/Combat.Combat")))))

(fn `UserConstructionScript`)