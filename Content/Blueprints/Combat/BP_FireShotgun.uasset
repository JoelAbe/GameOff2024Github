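; BP_FireShotgun is a short-lived fire shotgun spell actor used by either the player or the cave troll, branching on its owner.
; Player casts gather overlapping NPCs after a brief delay, apply spell-table damage and play impact audio.
; Troll casts reposition the box, opening a brief window for one AIDamage hit on the player via overlap.
; Effect fade-out and destruction follow player casts, but troll casts only on overlap.
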(event `self.ReceiveBeginPlay`
  (bind _box (`self.Box`))
  (`ActorComponent.Activate` (`self.NS_SpellEffect`) false)
  (`self.DetermineOwner`)
  (if (`self.TrollIsOwner`)
    (`SceneComponent.SetRelativeScale3D` _box (1.0 1.0 1.0))
    (`SceneComponent.K2_SetRelativeLocation` _box (1009.0 0.0 40.0) false false)
    (set `self.CanDamage` true)
    (`KismetSystemLibrary.K2_SetTimerDelegate` (delegate `StopAllowDamage`) 0.1)
    (else
      (`KismetSystemLibrary.Delay` 0.1)
      (if (not (`self.TrollIsOwner`))
        (for _array_element (`PrimitiveComponent.GetOverlappingActors` (`self.Box`) "/Script/CommonUI_FPSBase.NPCBaseCharacter")
          (`KismetArrayLibrary.Array_AddUnique` (`self.OverlappedActors`) _array_element))
        (set `self.CanDamage` true)
        (`KismetSystemLibrary.K2_SetTimerForNextTickDelegate` (delegate `StopDamage`))
        (`self.DealDamage`)))))

(event `StopDamage`
  (set `self.CanDamage` false))

(event `StopAllowDamage`
  (set `self.CanDamage` false))

(event `self.Box.OnComponentBeginOverlap`
  (params (OverlappedComponent :type "PrimitiveComponent Object Reference") (OtherActor :type "Actor Object Reference") (OtherComp :type "PrimitiveComponent Object Reference") (OtherBodyIndex :type Integer) (bFromSweep :type Boolean) (SweepResult :type "HitResult Structure (by ref)"))
  (set `self.Other Actor` OtherActor)
  (if (`self.TrollIsOwner`)
    (`self.Damage Player`)
    (`KismetSystemLibrary.Delay` 5.0)
    (`ActorComponent.Deactivate` (`self.NS_SpellEffect`))
    (`KismetSystemLibrary.Delay` 2.0)
    (`self.K2_DestroyActor`)))

(event `DealDamage`
  (for _array_element (`self.OverlappedActors`)
    (`self.DamageNPC` _array_element)
    (`AkGameplayStatics.PostEventAtLocation` "/Game/WwiseAudio/VortexImpact.VortexImpact" (`self.K2_GetActorLocation`) (`KismetMathLibrary.Conv_VectorToRotator` (`self.GetActorForwardVector`))))
  (`KismetSystemLibrary.Delay` 5.0)
  (`ActorComponent.Deactivate` (`self.NS_SpellEffect`))
  (`KismetSystemLibrary.Delay` 2.0)
  (`self.K2_DestroyActor`))

(fn `Damage Player`
  (if (not (`self.TookDamage`))
    (cast `/Game/Player/BP_JamPlayerCharacter` (`self.Other Actor`))
    (if (`self.CanDamage`)
      (`GameplayStatics.ApplyDamage` (`self.Other Actor`) (`self.AIDamage`) (`self.GetInstigatorController`) self)
      (set `self.TookDamage` true))))

(fn `DamageNPC`
  (params (DamagedActor :type "Actor Object Reference"))
  (bind _asnpcbase_character (cast `NPCBaseCharacter` DamagedActor))
  (bind _returnvalue (`|GetDataTableRow` "/Game/Game/Data/DT_Spells.DT_Spells" "3")
    (:`then`
      (if (`self.CanDamage`)
        (`GameplayStatics.ApplyDamage` _asnpcbase_character (`.BaseDamage` (break `Spell` _returnvalue)) (`self.GetInstigatorController`) self)))))

(fn `DetermineOwner`
  (bind _asbp_cave_troll (cast `/Game/NPCs/CaveTroll/BP_CaveTroll` (`self.ActorOwner`))
    (:`then`
      (set `self.As BP Cave Troll` _asbp_cave_troll)
      (set `self.TrollIsOwner` true))
    (:`CastFailed`
      (bind _asbp_jam_player_character (cast `/Game/Player/BP_JamPlayerCharacter` (`self.ActorOwner`)))
      (set `self.As BP Jam Player Character` _asbp_jam_player_character)
      (set `self.TrollIsOwner` false))))

(fn `UserConstructionScript`)