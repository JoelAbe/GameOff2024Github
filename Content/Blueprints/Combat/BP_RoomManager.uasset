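; Room manager that runs a combat encounter, spawning enemies when its linked combat trigger fires and reporting back when all are dead.
; A looping timer spawns one enemy per tick at random spawn points: gremlins (light), then mages (medium), then melee skeletons (heavy).
; Each enemy's death event decrements a counter preset to the planned total, and at zero the manager calls OnCombatComplete on the trigger.
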(event `self.ReceiveBeginPlay`
  (`/Engine/EditorBlueprintResources/StandardMacros.IsValid` (`self.LinkedCombatTrigger`)
    (:`Is Valid`
      (add `/Game/Blueprints/Combat/BP_CombatTrigger.OnCombatTriggered` (`self.LinkedCombatTrigger`) (delegate `OnCombatTriggered_Event`))
      (set `self.TotalEnemiesSpawned` (+ (`self.LightEnemiesToSpawn`) (`self.MediumEnemiesToSpawn`) (`self.HeavyEnemiesToSpawn`))))
    (:`Is Not Valid`
      (`KismetSystemLibrary.PrintString` "No combat trigger linked, spawning will fail" true true (struct :`R` 1.0 :`G` 0.008603 :`A` 1.0) 10.0))))

(event `OnCombatTriggered_Event`
  (bind _returnvalue (`KismetSystemLibrary.K2_SetTimerDelegate` (delegate `SpawnWave`) 0.4 true))
  (set `self.SpawnEnemiesTimerHandle` _returnvalue))

(event `SpawnWave`
  (if (and (> (`self.LightEnemiesToSpawn`) 0) (< (`self.LightEnemiesSpawned`) (`self.LightEnemiesToSpawn`)))
    (bind _spawnedenemy (`self.SpawnLightEnemy`))
    (add `NPCBaseCharacter.OnNPCDeath` _spawnedenemy (delegate `OnNPCDeath_Event`))
    (elif (and (> (`self.MediumEnemiesToSpawn`) 0) (< (`self.MediumEnemiesSpawned`) (`self.MediumEnemiesToSpawn`)))
      (bind _spawnedenemy_2 (`self.SpawnMediumEnemy`))
      (add `NPCBaseCharacter.OnNPCDeath` _spawnedenemy_2 (delegate `OnNPCDeath_Event`))
      (elif (and (> (`self.HeavyEnemiesToSpawn`) 0) (< (`self.HeavyEnemiesSpawned`) (`self.HeavyEnemiesToSpawn`)))
        (bind _spawnedenemy_3 (`self.SpawnHeavyEnemy`))
        (add `NPCBaseCharacter.OnNPCDeath` _spawnedenemy_3 (delegate `OnNPCDeath_Event`))
        (else
          (`KismetSystemLibrary.K2_ClearAndInvalidateTimerHandle` (`self.SpawnEnemiesTimerHandle`)))))))

(event `OnNPCDeath_Event`
  (`/Engine/EditorBlueprintResources/StandardMacros.DecrementInt` (`self.TotalEnemiesSpawned`)
    (:`  `
      (`KismetSystemLibrary.PrintString` (`KismetStringLibrary.Conv_IntToString` (`self.TotalEnemiesSpawned`)))
      (if (<= (`self.TotalEnemiesSpawned`) 0)
        (`/Game/Blueprints/Combat/BP_CombatTrigger.OnCombatComplete` (`self.LinkedCombatTrigger`))))))

(fn `SpawnHeavyEnemy`
  (returns (SpawnedEnemy :type "NPCBaseCharacter Object Reference"))
  (bind _returnvalue (`|SpawnActorFromClass` "/Game/NPCs/MeleeSkeleton/BP_MeleeSkeleton.BP_MeleeSkeleton_C" (`KismetMathLibrary.MakeTransform` (`self.K2_GetActorLocation` (`KismetArrayLibrary.Array_Random` (`self.SpawnPoints`)))) "AlwaysSpawn" "MultiplyWithRoot" null self null))
  (`/Engine/EditorBlueprintResources/StandardMacros.IncrementInt` (`self.HeavyEnemiesSpawned`)
    (:`  `
      (return _returnvalue))))

(fn `SpawnLightEnemy`
  (returns (SpawnedEnemy :type "NPCBaseCharacter Object Reference"))
  (`/Engine/EditorBlueprintResources/StandardMacros.IncrementInt` (`self.LightEnemiesSpawned`)
    (:`  `
      (bind _returnvalue (`|SpawnActorFromClass` "/Game/NPCs/Gremlin/BP_Gremlin.BP_Gremlin_C" (`KismetMathLibrary.MakeTransform` (`self.K2_GetActorLocation` (`KismetArrayLibrary.Array_Random` (`self.SpawnPoints`)))) "Undefined" "MultiplyWithRoot" null self null))
      (return _returnvalue))))

(fn `SpawnMediumEnemy`
  (returns (SpawnedEnemy :type "NPCBaseCharacter Object Reference"))
  (bind _returnvalue (`|SpawnActorFromClass` "/Game/NPCs/Mage/BP_MageNPC.BP_MageNPC_C" (`KismetMathLibrary.MakeTransform` (`self.K2_GetActorLocation` (`KismetArrayLibrary.Array_Random` (`self.SpawnPoints`)))) "AlwaysSpawn" "MultiplyWithRoot" null self null))
  (`/Engine/EditorBlueprintResources/StandardMacros.IncrementInt` (`self.MediumEnemiesSpawned`)
    (:`  `
      (return _returnvalue))))

(fn `UserConstructionScript`)