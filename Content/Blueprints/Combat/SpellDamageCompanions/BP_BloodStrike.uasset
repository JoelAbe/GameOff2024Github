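; Blood Strike spell companion actor that gives the player lifesteal from nearby NPC health loss.
; On BeginPlay it plays the BloodCast Wwise sound, then totals the health of NPCs overlapping its sphere at two delayed moments.
; Half of any drop between the totals is added to the player's health.
; It applies no damage itself and re-queries overlaps, so NPCs entering or leaving the sphere skew the result.
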(event `self.ReceiveBeginPlay`
  (bind _returnvalue (/ (- (`self.PreDamageHealth`) (`self.PostDamageHealth`)) 2.0))
  (`AkGameplayStatics.PostEventAtLocation` "/Game/WwiseAudio/BloodCast.BloodCast" (`self.K2_GetActorLocation`) (`KismetMathLibrary.Conv_VectorToRotator` (`self.GetActorForwardVector`)))
  (set `self.Player Character Ref` (`/Game/Blueprints/BFL_CommonFunctions.GetPlayerCharacterRef`))
  (`KismetSystemLibrary.Delay` (/ (`self.InitialDelay`) 2.0))
  (for _array_element (`PrimitiveComponent.GetOverlappingActors` (`self.CollisionSphere`) "/Script/CommonUI_FPSBase.NPCBaseCharacter")
    (bind _asnpcbase_character (cast `NPCBaseCharacter` _array_element))
    (bind _returnvalue_2 (`AttributesComponent.GetCurrentHealth` (`NPCBaseCharacter.CharacterAttributes` _asnpcbase_character)))
    (set `self.PreDamageHealth` (+ (`self.PreDamageHealth`) _returnvalue_2)))
  (`KismetSystemLibrary.PrintString` (`KismetStringLibrary.Conv_DoubleToString` (`self.PreDamageHealth`)))
  (`KismetSystemLibrary.Delay` (`self.InitialDelay`))
  (for _array_element_2 (`PrimitiveComponent.GetOverlappingActors` (`self.CollisionSphere`) "/Script/CommonUI_FPSBase.NPCBaseCharacter")
    (bind _asnpcbase_character_2 (cast `NPCBaseCharacter` _array_element_2))
    (bind _returnvalue_3 (`AttributesComponent.GetCurrentHealth` (`NPCBaseCharacter.CharacterAttributes` _asnpcbase_character_2)))
    (set `self.PostDamageHealth` (+ (`self.PostDamageHealth`) _returnvalue_3)))
  (`KismetSystemLibrary.PrintString` (`KismetStringLibrary.Conv_DoubleToString` (`self.PostDamageHealth`)))
  (if (> _returnvalue 0.0)
    (`AttributesComponent.AddHealth` (`JamPlayerCharacter.Attributes` (`self.Player Character Ref`)) _returnvalue)
    (`KismetSystemLibrary.PrintString` (`KismetStringLibrary.Conv_DoubleToString` _returnvalue))))

(fn `UserConstructionScript`)