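; BP_RainTrigger is a trigger volume that changes the Ultra Dynamic Weather state when the player enters it.
; On BeginPlay it finds and caches the Ultra Dynamic Weather reference.
; When the player character overlaps its box, it sets the weather to Rain if EnableRainEffect is true, otherwise to Foggy.
; Leaving the box does not revert the weather.
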(event `self.ReceiveBeginPlay`
  (bind _udw (`/Game/UltraDynamicSky/Blueprints/Functions/UltraDynamicWeather_Functions.Get Ultra Dynamic Weather`))
  (set `self.UDW` _udw))

(event `self.Box.OnComponentBeginOverlap`
  (params (OverlappedComponent :type "PrimitiveComponent Object Reference") (OtherActor :type "Actor Object Reference") (OtherComp :type "PrimitiveComponent Object Reference") (OtherBodyIndex :type Integer) (bFromSweep :type Boolean) (SweepResult :type "HitResult Structure (by ref)"))
  (bind _udw (`self.UDW`))
  (if (== OtherActor (`GameplayStatics.GetPlayerCharacter` 0))
    (if (`self.EnableRainEffect`)
      (set `/Game/UltraDynamicSky/Blueprints/Ultra_Dynamic_Weather.Weather` "/Game/UltraDynamicSky/Blueprints/Weather_Effects/Weather_Presets/Rain.Rain" _udw)
      (else
        (set `/Game/UltraDynamicSky/Blueprints/Ultra_Dynamic_Weather.Weather` "/Game/UltraDynamicSky/Blueprints/Weather_Effects/Weather_Presets/Foggy.Foggy" _udw)))))

(fn `UserConstructionScript`)