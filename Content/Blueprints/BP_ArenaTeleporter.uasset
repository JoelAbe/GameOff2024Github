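; BP_ArenaTeleporter is a portal actor that moves the player character when it enters the overlap sphere.
; It caches player 0's character on BeginPlay and ignores other overlapping actors.
; On overlap it applies TeleportLocation's relative location as the player's world location and its relative rotation as control rotation.
; It then plays a 2D sound and briefly pulses PortalCloseEffect.
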(event `self.ReceiveBeginPlay`
  (set `self.PlayerRef` (`GameplayStatics.GetPlayerCharacter` 0)))

(event `self.OverlapSphere.OnComponentBeginOverlap`
  (params (OverlappedComponent :type "PrimitiveComponent Object Reference") (OtherActor :type "Actor Object Reference") (OtherComp :type "PrimitiveComponent Object Reference") (OtherBodyIndex :type Integer) (bFromSweep :type Boolean) (SweepResult :type "HitResult Structure (by ref)"))
  (bind _teleportlocation (`self.TeleportLocation`))
  (bind _portalcloseeffect (`self.PortalCloseEffect`))
  (if (== OtherActor (`self.PlayerRef`))
    (`self.K2_SetActorLocation` (`self.PlayerRef`) (`SceneComponent.RelativeLocation` _teleportlocation) false false)
    (`Controller.SetControlRotation` (`GameplayStatics.GetPlayerController` 0) (`SceneComponent.RelativeRotation` _teleportlocation))
    ;[1 1 1] TP Sound
    (`GameplayStatics.PlaySound2D` null 1.0 1.0 0.0 null null)
    (`ActorComponent.Activate` _portalcloseeffect false)
    (`KismetSystemLibrary.Delay` 0.1)
    (`ActorComponent.Deactivate` _portalcloseeffect)))

(fn `UserConstructionScript`)