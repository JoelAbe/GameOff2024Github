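; Player controller that owns the gameplay UI: HUD, pause menu and spell wheel.
; Outside MainMenuMap, BeginPlay creates a master widget, pushes the HUD and listens for StacksCleared to reset the Escape toggle.
; Escape toggles the pause menu only when it is active or the menu stack is empty.
; Holding Control shows the spell wheel on the menu stack, blocked while the player is dead or charging.
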(event `self.ReceiveBeginPlay`
  (bind _returnvalue (`GameplayStatics.GetCurrentLevelName` true))
  (if (not (`KismetStringLibrary.EqualEqual_StrStr` _returnvalue "MainMenuMap"))
    (`self.CreateAndPushStartingWidgets`)
    ;[0 0 0] Assign callback function to BaseWidget's broadcast event "StacksCleared"
    (add `/Game/UI/Common/Widgets/WB_MasterWidget.OnStacksCleared` (`self.MasterWidgetRef`) (delegate `OnStacksCleared_Event`))
    (set `self.Player Character Ref` (`/Game/Blueprints/BFL_CommonFunctions.GetPlayerCharacterRef`))
    (`/Game/UI/Common/Widgets/WB_MasterWidget.SetInputMode_MenuClosed` (`self.MasterWidgetRef`))))

(event `OnStacksCleared_Event`
  ;[0 0 0] Assign callback function to BaseWidget's broadcast event "StacksCleared"
  (set `self.isEscActivated` false))

(event `EnhancedInput|/Game/Player/Input/InputActions/IA_Escape`
  (params (ActionValue :type Boolean) (ElapsedSeconds :type "Float (double-precision)") (TriggeredSeconds :type "Float (double-precision)") (InputAction :type "InputAction Object Reference" :default "/Game/Player/Input/InputActions/IA_Escape.IA_Escape"))
  (:`Started`
    (`self.HandlePauseMenu`)))

(event `EnhancedInput|/Game/Player/Input/InputActions/IA_Control`
  (params (ActionValue :type Boolean) (ElapsedSeconds :type "Float (double-precision)") (TriggeredSeconds :type "Float (double-precision)") (InputAction :type "InputAction Object Reference" :default "/Game/Player/Input/InputActions/IA_Control.IA_Control"))
  (bind _player_character_ref (`self.Player Character Ref`))
  (bind _pushedwidget (`/Game/UI/Common/Widgets/WB_MasterWidget.PushedWidget` (`self.MasterWidgetRef`)))
  (bind _returnvalue (and (not (`/Game/Player/BP_JamPlayerCharacter.isDead` _player_character_ref)) (not (`/Game/Player/BP_JamPlayerCharacter.isCharging` _player_character_ref)) (not (`/Game/Player/BP_JamPlayerCharacter.2hIsCharging` _player_character_ref))))
  (:`Started`
    (if _returnvalue
      ;[0 0 0] Push the widget (selected in the Activatable Widget Class dropdown) to the desired stack (in this case, the tab menu gets pushed to the Menu stack)
      (`/Game/UI/Common/Widgets/WB_MasterWidget.Push Widget to Target Stack` (`self.MasterWidgetRef`) (`/Game/UI/Common/Widgets/WB_MasterWidget.Menu_Stack` (`self.MasterWidgetRef`)) "/Game/UI/Common/Widgets/Menus/WB_SpellWheel.WB_SpellWheel_C" true false)))
  (:`Completed`
    (if _returnvalue
      (if (== (`GameplayStatics.GetObjectClass` _pushedwidget) "/Game/UI/Common/Widgets/Menus/WB_SpellWheel.WB_SpellWheel_C")
        (`/Game/UI/Common/Widgets/WB_MasterWidget.DeactivateWidget_Event` (`self.MasterWidgetRef`) _pushedwidget)))))

(fn `CreateAndPushStartingWidgets`
  (bind _returnvalue (`|CreateWidget` "/Game/UI/Common/Widgets/WB_MasterWidget.WB_MasterWidget_C" (`GameplayStatics.GetPlayerController` 0)))
  (bind _output_get (set `self.MasterWidgetRef` _returnvalue))
  (`UserWidget.AddToViewport` _output_get 0)
  (`/Game/UI/Common/Widgets/WB_MasterWidget.Push Widget to Target Stack` _output_get (`/Game/UI/Common/Widgets/WB_MasterWidget.HUD_Stack` _output_get) "/Game/UI/Common/Widgets/HUD/WB_MainHUD.WB_MainHUD_C" false false))

(fn `GetCurrentlyActiveWidgetClass`
  (returns (ReturnValue :type "CommonActivatableWidget Class Reference"))
  (return (`GameplayStatics.GetObjectClass` (`/Game/UI/Common/Widgets/WB_MasterWidget.PushedWidget` (`self.MasterWidgetRef`)))))

(fn `HandlePauseMenu`
  ;[0 0 0] If the pause menu is active OR the menu stack is clear, allow input from this input event
  (if (or (== (`self.GetCurrentlyActiveWidgetClass`) "/Game/UI/Common/Widgets/Menus/WB_PauseMenu.WB_PauseMenu_C") (`self.isMenuStackEmpty?`))
    ;[0 0 0] Starts false. when the player presses tab, this switches to true. when they press it again, it switches to false, etc. Also controls menu opening and closing, so if a menu gets closed somewhere else (and closing that menu returns the player to gameplay, not UI) set this back to false so menus work as expected on the next tab press (base widget checks for this but if something is bugged check this)
    (bind _output_get (set `self.isEscActivated` (not (`self.isEscActivated`))))
    ;[0 0 0] When isTabActivated is True, try to open the tab menu. When it's false, try to close it
    (if _output_get
      ;[0 0 0] Push the widget (selected in the Activatable Widget Class dropdown) to the desired stack (in this case, the tab menu gets pushed to the Menu stack)
      (`/Game/UI/Common/Widgets/WB_MasterWidget.Push Widget to Target Stack` (`self.MasterWidgetRef`) (`/Game/UI/Common/Widgets/WB_MasterWidget.Menu_Stack` (`self.MasterWidgetRef`)) "/Game/UI/Common/Widgets/Menus/WB_PauseMenu.WB_PauseMenu_C" true false)
      (else
        ;[0 0 0] Because we don't want Tab to close EVERY menu, just the one it opened (this one), check that the pause menu is the active widget, then deactivate it.
        (if (== (`self.GetCurrentlyActiveWidgetClass`) "/Game/UI/Common/Widgets/Menus/WB_PauseMenu.WB_PauseMenu_C")
          (`/Game/UI/Common/Widgets/WB_MasterWidget.DeactivateWidget_Event` (`self.MasterWidgetRef`) (`/Game/UI/Common/Widgets/WB_MasterWidget.PushedWidget` (`self.MasterWidgetRef`))))))))

(fn `isMenuStackEmpty?`
  (returns (isEmpty :type Boolean))
  (return (== (`/Game/UI/Common/Widgets/WB_MasterWidget.PushedWidget` (`self.MasterWidgetRef`)) null)))

(fn `UserConstructionScript`)