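; Player character for a spellcasting game, handling dash, interaction, health, mana, save-data restore and game over.
; Holding shoot charges the equipped spell on a timer; releasing fires it if charged, otherwise cancels.
; FireSpell spawns camera-aimed projectiles or conjures at a decal-previewed ground point, with shotgun, heal and other cases partly hardcoded by spell ID.
; Looping timers regenerate health and mana, updating the HUD, while Wwise events and camera shakes provide feedback.
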(event `EnhancedInput|/Game/Player/Input/InputActions/IA_Shift`
  (params (ActionValue :type Boolean) (ElapsedSeconds :type "Float (double-precision)") (TriggeredSeconds :type "Float (double-precision)") (InputAction :type "InputAction Object Reference" :default "/Game/Player/Input/InputActions/IA_Shift.IA_Shift"))
  (:`Started`
    (if (and (not (`self.isCharging`)) (not (`self.2hIsCharging`)))
      (`self.StartDash`)
      (if (`self.isDashing`)
        (`AkGameplayStatics.PostEvent` "/Game/WwiseAudio/Dash.Dash" self)
        (`self.PlayCameraShake` "/Game/Blueprints/CameraShakes/BP_DashShake.BP_DashShake_C")))))

(event `self.ReceiveTick`
  (params (DeltaSeconds :type "Float (single-precision)"))
  (bind _interacttext (`/Game/UI/Common/Widgets/HUD/WB_MainHUD.InteractText` (`/Game/Player/BP_JamPlayerState.HUDRef` (`self.BP Player State Ref`))))
  (if (`self.ReferencesSet`)
    (`self.UpdateDashWidget`)
    (`/Engine/EditorBlueprintResources/StandardMacros.IsValid` (`self.LookAtActor`)
      (:`Is Valid`
        (`Widget.SetRenderOpacity` _interacttext 1.0))
      (:`Is Not Valid`
        (if (not (<= (`Widget.RenderOpacity` _interacttext) 0.0))
          (`Widget.SetRenderOpacity` _interacttext 0.0))))))

(event `EnhancedInput|/Game/Player/Input/InputActions/IA_Jump`
  (params (ActionValue :type Boolean) (ElapsedSeconds :type "Float (double-precision)") (TriggeredSeconds :type "Float (double-precision)") (InputAction :type "InputAction Object Reference" :default "/Game/Player/Input/InputActions/IA_Jump.IA_Jump")))

(event `self.OnLanded`
  (params (Hit :type "HitResult Structure (by ref)"))
  (`AkGameplayStatics.PostEvent` "/Game/WwiseAudio/JumpLand.JumpLand" self)
  (set `self.isDoubleJumping` false)
  (`self.PlayCameraShake` "/Game/Blueprints/CameraShakes/BP_OnLandedShake.BP_OnLandedShake_C")
  (`/Engine/EditorBlueprintResources/StandardMacros.DoOnce` false :!via `Reset`
    (:`Completed`
      (`self.LaunchCharacter` (0.0 0.0 700.0) false true))))

(event `self.OnDamageReceived`
  (bind _attributes (`self.Attributes`))
  (`self.SetHealthWidget`)
  (`self.StartHealthRecharge`)
  (`AkGameplayStatics.PostEvent` "/Game/WwiseAudio/DamageDealt.DamageDealt" self)
  (if (< (`AttributesComponent.Health` _attributes) (/ (`AttributesComponent.MaxHealth` _attributes) 2.0))
    (if (not (`KismetSystemLibrary.IsValid` (`AkGameObject.AkAudioEvent` (`self.AK_Heartbeat`))))
      (`self.PlayNewAKSound` "/Game/WwiseAudio/HeartbeatDamaged.HeartbeatDamaged" (`self.AK_Heartbeat`)))))

(event `StartHealthRecharge`
  (bind _returnvalue (`KismetSystemLibrary.K2_SetTimerDelegate` (delegate `RechargeHealth`) (`self.HealthChargeRate`) true))
  (set `self.RechargeHealthTimerHandle` _returnvalue))

(event `RechargeHealth`
  (bind _attributes (`self.Attributes`))
  (bind _ak_heartbeat (`self.AK_Heartbeat`))
  (bind _attributes_2 (`self.Attributes`))
  (`AttributesComponent.AddHealth` (`self.Attributes`) (`self.HealthChargeAmountPerTick`))
  (`self.SetHealthWidget`)
  (if (> (`AttributesComponent.Health` _attributes_2) (/ (`AttributesComponent.MaxHealth` _attributes_2) 2.0))
    (`AkGameObject.Stop` _ak_heartbeat)
    (set `AkGameObject.AkAudioEvent` null _ak_heartbeat))
  (if (>= (`AttributesComponent.Health` _attributes) (`AttributesComponent.MaxHealth` _attributes))
    (`KismetSystemLibrary.K2_ClearAndInvalidateTimerHandle` (`self.RechargeHealthTimerHandle`))))

(event `OnManaLost`
  (bind _returnvalue (`KismetSystemLibrary.K2_SetTimerDelegate` (delegate `RechargeMana`) (`self.ManaChargeRate`) true))
  (set `self.ManaChargeTimerHandle` _returnvalue))

(event `RechargeMana`
  (bind _attributes (`self.Attributes`))
  (`AttributesComponent.AddMana` (`self.Attributes`) (`self.ManaChargeAmountPerTick`))
  (`self.SetManaWidget`)
  (if (>= (`AttributesComponent.Mana` _attributes) (`AttributesComponent.MaxMana` _attributes))
    (`KismetSystemLibrary.K2_ClearAndInvalidateTimerHandle` (`self.ManaChargeTimerHandle`))))

(event `self.OnPlayerDataLoaded`
  (bind _bp_player_state_ref (`self.BP Player State Ref`))
  (bind _attributes (`self.Attributes`))
  (bind _attributes_2 (`self.Attributes`))
  (set `self.DataLoaded` true)
  (`KismetSystemLibrary.Delay` 0.2)
  (`/Game/Player/BP_JamPlayerState.SetEquippedSpell` _bp_player_state_ref (`JamPlayerState.EquippedSpell` _bp_player_state_ref))
  (if (< (`AttributesComponent.Health` _attributes_2) (`AttributesComponent.MaxHealth` _attributes_2))
    (`self.StartHealthRecharge`))
  (if (< (`AttributesComponent.Mana` _attributes) (`AttributesComponent.MaxMana` _attributes))
    (`self.OnManaLost`)))

(event `self.ReceiveBeginPlay`
  (`KismetSystemLibrary.Delay` 0.5)
  (`self.SetReferences`)
  (bind _returnvalue (message `SaveGameInterface.GetSaveGameData` (subsystem `JamGameInstanceSubsystem`)))
  (`/Engine/EditorBlueprintResources/StandardMacros.IsValid` _returnvalue
    (:`Is Valid`
      (`self.SetPlayerStateFromSaveData` (`JamSaveGameObject.PlayerData` _returnvalue))
      (`self.SetHealthWidget`)
      (`self.SetManaWidget`))
    (:`Is Not Valid`
      (`AttributesComponent.InitializeAttributeValues` (`self.Attributes`))
      (`self.SetHealthWidget`)
      (`self.SetManaWidget`))))

(event `self.OnDeath`
  (bind _masterwidgetref (`/Game/Player/BP_JamPlayerController.MasterWidgetRef` (`self.Player Controller Ref`)))
  (set `self.isDead` true)
  (`/Game/UI/Common/Widgets/WB_MasterWidget.Push Widget to Target Stack` _masterwidgetref (`/Game/UI/Common/Widgets/WB_MasterWidget.Menu_Stack` _masterwidgetref) "/Game/UI/Common/Widgets/Menus/WB_GameOverMenu.WB_GameOverMenu_C" true false)
  (`GameplayStatics.SetGlobalTimeDilation` 0.0)
  (`AkGameplayStatics.SetState` "/Game/WwiseAudio/SetStates/PlayerDeath.PlayerDeath"))

(event `EnhancedInput|/Game/Player/Input/InputActions/IA_Shoot`
  (params (ActionValue :type Boolean) (ElapsedSeconds :type "Float (double-precision)") (TriggeredSeconds :type "Float (double-precision)") (InputAction :type "InputAction Object Reference" :default "/Game/Player/Input/InputActions/IA_Shoot.IA_Shoot"))
  (bind _bp_player_state_ref (`self.BP Player State Ref`))
  (bind _bp_player_state_ref_2 (`self.BP Player State Ref`))
  (bind (_id _name _spelltype _icon _description _isvalid _istwohanded _chargetime) (break `Spell` (`JamPlayerState.EquippedSpell` _bp_player_state_ref)))
  ;[0 0 0] Cast spell
  (:`Triggered`
    (if (or (`self.isCharging`) (`self.2hIsCharging`))
      (`self.PlayCameraShake` "/Game/Blueprints/CameraShakes/Spells/BP_ChargeSpellShake.BP_ChargeSpellShake_C")
      (`/Engine/EditorBlueprintResources/StandardMacros.IsValid` _bp_player_state_ref_2
        (:`Is Valid`
          (if (and (`|EnumEquality` (`.SpellType` (break `Spell` (`JamPlayerState.EquippedSpell` _bp_player_state_ref_2))) "Conjure") (`self.isCharging`))
            (`self.CalculateConjureLocation`))))))
  (:`Started`
    (`/Engine/EditorBlueprintResources/StandardMacros.IsValid` _bp_player_state_ref
      (:`Is Valid`
        (`self.CheckMana`)
        (if (and _isvalid (`self.CanCastSpell`))
          ;;[0 0 0] Start charging the spell
          (`self.StartSpell`)
          (bind _returnvalue (`KismetSystemLibrary.K2_SetTimer` null "ChargeSpell" _chargetime))
          (set `self.ChargeTimerHandle` _returnvalue)
          (bind _returnvalue_2 (`|CreateWidget` "/Game/UI/Common/Widgets/Popups/WB_SpellChargeProgressBar.WB_SpellChargeProgressBar_C" (`self.PlayerController`)))
          (bind _output_get (set `self.SpellChargeWidget` _returnvalue_2))
          (`UserWidget.AddToViewport` _output_get -1)
          (bind _returnvalue_3 (`KismetSystemLibrary.K2_SetTimerDelegate` (delegate `UpdateSpellProgressbar`) (`GameplayStatics.GetWorldDeltaSeconds`) true))
          (set `self.ChargeProgressBarTimerHandle` _returnvalue_3)
          (`self.PlayNewAKSound` (`.SpellChargeSound` (break `Spell` (`JamPlayerState.EquippedSpell` (`self.BP Player State Ref`)))) (`self.Ak_SpellCharge`))))))
  (:`Completed`
    (if (`self.isCharged`)
      (`self.RemoveSpellChargeWidget`)
      ;;[0 0 0] Controls animations and walk speed
      (`self.FinishSpell`)
      (`KismetSystemLibrary.Delay` 0.1)
      (`self.FireSpell`)
      (else
        (`self.CancelSpell`)
        (`self.ClearChargeTimer`)))))

(event `UpdateSpellProgressbar`
  ;[0 0 0] Cast spell
  (set `self.SpellChargeProgress` (/ (`KismetSystemLibrary.K2_GetTimerElapsedTimeHandle` (`self.ChargeTimerHandle`)) (`.ChargeTime` (break `Spell` (`JamPlayerState.EquippedSpell` (`self.BP Player State Ref`))))))
  (if (`self.isCharged`)
    (set `self.SpellChargeProgress` 1.0)))

(event `EnhancedInput|/Game/Player/Input/InputActions/IA_RightClick`
  (params (ActionValue :type Boolean) (ElapsedSeconds :type "Float (double-precision)") (TriggeredSeconds :type "Float (double-precision)") (InputAction :type "InputAction Object Reference" :default "/Game/Player/Input/InputActions/IA_RightClick.IA_RightClick"))
  (:`Started`
    (`self.CancelSpell`)
    (`self.ClearChargeTimer`))
  (:`Completed`
    (set `self.SpellCancelled` false)))

(event `EnhancedInput|/Game/Player/Input/InputActions/IA_E`
  (params (ActionValue :type Boolean) (ElapsedSeconds :type "Float (double-precision)") (TriggeredSeconds :type "Float (double-precision)") (InputAction :type "InputAction Object Reference" :default "/Game/Player/Input/InputActions/IA_E.IA_E"))
  (bind _lookatactor (`self.LookAtActor`))
  ;[0 0 0] Draws a line from the camera to a point [InteractDistance] away, checks if the hit actor implements the interact interface. If it did, call its interact function
  (:`Started`
    (message `InteractInterface.Interact` _lookatactor)
    (`/Engine/EditorBlueprintResources/StandardMacros.IsValid` _lookatactor
      (:`Is Valid`
        (if (`self.ActorHasTag` (`self.LookAtActor`) "Glyph")
          (`|PlayMontage` (`self.SkeletalMesh`) "/Game/MedievalArmour/RetargetedAnimations/WizardArmsWithGloves/L_PalmBlast_Start_Montage.L_PalmBlast_Start_Montage" 2.0))))))

(fn `CalculateConjureLocation`
  (bind _camera (`self.Camera`))
  (bind _returnvalue (`SceneComponent.K2_GetComponentLocation` _camera))
  (bind (_outhit _returnvalue_2) (`KismetSystemLibrary.LineTraceSingleForObjects` _returnvalue (+ _returnvalue (* (`SceneComponent.GetForwardVector` _camera) (`self.ConjureDistance`))) (`|MakeArray` "ObjectTypeQuery1" "ObjectTypeQuery2" :!type "EObjectTypeQuery Enum")))
  (bind (_bblockinghit _binitialoverlap _time _distance _location _impactpoint _normal _impactnormal _physmat _hitactor _hitcomponent _hitbonename _bonename _hititem _elementindex _faceindex _tracestart _traceend) (`GameplayStatics.BreakHitResult` _outhit))
  (bind _returnvalue_3 (`KismetMathLibrary.SelectVector` _impactpoint _traceend _returnvalue_2))
  (bind (_outhit_2 _returnvalue_4) (`KismetSystemLibrary.LineTraceSingleForObjects` (+ _returnvalue_3 (0.0 0.0 200.0)) (- _returnvalue_3 (0.0 0.0 1000.0)) (`|MakeArray` "ObjectTypeQuery1" "ObjectTypeQuery2" :!type "EObjectTypeQuery Enum")))
  (if _returnvalue_4
    (bind (_bblockinghit_2 _binitialoverlap_2 _time_2 _distance_2 _location_2 _impactpoint_2) (`GameplayStatics.BreakHitResult` _outhit_2))
    (`GameplayStatics.SpawnDecalAtLocation` "/Game/Materials/M_MagicCircleDecal.M_MagicCircleDecal" (`.SpellDecalSize` (break `Spell` (`JamPlayerState.EquippedSpell` (`self.BP Player State Ref`)))) _impactpoint_2 (struct :`Pitch` -90.0) (`GameplayStatics.GetWorldDeltaSeconds`))
    (set `self.ConjureLocation` _impactpoint_2)))

(fn `CancelSpell`
  (set `self.SpellCancelled` true)
  (set `self.isCharging` false)
  (set `self.isCharged` false)
  (set `self.2hIsCharging` false)
  (set `self.2hFiredProjectile` false)
  (`self.RemoveSpellChargeWidget`)
  (set `CharacterMovementComponent.MaxWalkSpeed` (`self.DefaultWalkSpeed`) (`self.CharacterMovement`))
  (`AkGameObject.Stop` (`self.Ak_SpellCharge`)))

(fn `CastHealSpell`
  (`NiagaraFunctionLibrary.SpawnSystemAtLocation` "/Game/MagicAbilitiesVol2/Particles/NiagaraSystems/NS_ImpactAoE09_Heal.NS_ImpactAoE09_Heal" (- (`self.K2_GetActorLocation`) (0.0 0.0 90.0)) (struct) (2.0 2.0 2.0))
  (`AttributesComponent.AddHealth` (`self.Attributes`) (`self.HealAmount`))
  (`self.SetHealthWidget`))

(fn `ChargeSpell`
  (set `self.isCharged` true))

(fn `CheckMana`
  (bind _hudref (`/Game/Player/BP_JamPlayerState.HUDRef` (`self.BP Player State Ref`)))
  (bind _output_get (set `self.CanCastSpell` (or (>= (`AttributesComponent.Mana` (`self.Attributes`)) (`.ManaCost` (break `Spell` (`JamPlayerState.EquippedSpell` (`self.BP Player State Ref`))))) (== (`.ID` (break `Spell` (`JamPlayerState.EquippedSpell` (`self.BP Player State Ref`)))) 1))))
  (if (not _output_get)
    (`UserWidget.PlayAnimation` _hudref (`/Game/UI/Common/Widgets/HUD/WB_MainHUD.OutOfMana` _hudref) 0.0 1 "Forward" 1.0 false)))

(fn `ClearChargeTimer`
  (bind _chargetimerhandle (`self.ChargeTimerHandle`))
  (if (`KismetSystemLibrary.K2_IsValidTimerHandle` _chargetimerhandle)
    (`KismetSystemLibrary.K2_ClearAndInvalidateTimerHandle` _chargetimerhandle)))

(fn `FinishSpell`
  (set `self.isCharged` false)
  (set `self.isCharging` false)
  (set `self.SpellChargeProgress` 0.0)
  (set `CharacterMovementComponent.MaxWalkSpeed` (`self.DefaultWalkSpeed`) (`self.CharacterMovement`))
  (`AttributesComponent.RemoveMana` (`self.Attributes`) (`.ManaCost` (break `Spell` (`JamPlayerState.EquippedSpell` (`self.BP Player State Ref`)))))
  (`self.OnManaLost`)
  (`self.SetManaWidget`)
  (switch `ESpellType` (`self.CurrentSpell`)
    (:`TwoHanded`
      (set `self.2hFiredProjectile` true)
      (set `self.2hIsCharging` false))
    (:`Beam`
      (set `self.FiredProjectile` true :!label _label))
    (:`Projectile`
      (goto _label))
    (:`Conjure`
      (goto _label))))

(fn `FireSpell`
  (bind _returnvalue (`self.GetActorForwardVector`))
  (bind (_returnvalue_x _returnvalue_y) (`KismetMathLibrary.BreakVector2D` (`WidgetLayoutLibrary.GetViewportSize`)))
  (bind _conjurelocation (`self.ConjureLocation`))
  (bind _returnvalue_location (`KismetMathLibrary.BreakTransform` (`SceneComponent.GetSocketTransform` (`self.SkeletalMesh`) "HandProjectileSocket" "RTS_World")))
  (bind _equippedspell (`JamPlayerState.EquippedSpell` (`self.BP Player State Ref`)))
  (bind (_id _name _spelltype _icon _description _isvalid _istwohanded _chargetime _idleparticleeffect _projectileclass _basedamage) (break `Spell` _equippedspell))
  (bind (_id_2 _name_2 _spelltype_2 _icon_2 _description_2 _isvalid_2 _istwohanded_2 _chargetime_2 _idleparticleeffect_2 _projectileclass_2 _basedamage_2 _manacost _spellidlesound _spellchargesound _spellfiresound _spelldecalsize _damagecompanion) (break `Spell` (`JamPlayerState.EquippedSpell` (`self.BP Player State Ref`))))
  (bind (_worldposition _worlddirection) (`GameplayStatics.DeprojectScreenToWorld` (`GameplayStatics.GetPlayerController` 0) (`KismetMathLibrary.MakeVector2D` (/ _returnvalue_x 2.0) (/ _returnvalue_y 2.0))))
  (if (`KismetSystemLibrary.IsValidClass` (`.ProjectileClass` (break `Spell` (`JamPlayerState.EquippedSpell` (`self.BP Player State Ref`)))))
    (bind (_outhit _returnvalue_2) (`KismetSystemLibrary.LineTraceSingle` _worldposition (* _worlddirection 500000.0) "TraceTypeQuery2"))
    (bind (_bblockinghit _binitialoverlap _time _distance _location _impactpoint _normal _impactnormal _physmat _hitactor _hitcomponent _hitbonename _bonename _hititem _elementindex _faceindex _tracestart _traceend) (`GameplayStatics.BreakHitResult` _outhit))
    (bind _returnvalue_3 (`|SpawnActorFromClass` _projectileclass (`KismetMathLibrary.MakeTransform` _returnvalue_location (`KismetMathLibrary.FindLookAtRotation` _returnvalue_location (`KismetMathLibrary.SelectVector` _impactpoint _traceend _returnvalue_2))) "AlwaysSpawn" "MultiplyWithRoot" self _basedamage _equippedspell true (`self.GetInstigator`)))
    (`MagicProjectile.LaunchProjectile` _returnvalue_3)
    (set `self.ProjectileForwardVector` (`self.GetActorForwardVector`))
    (`AkGameObject.Stop` (`self.Ak_SpellCharge`))
    (`self.PlayCameraShake` "/Game/Blueprints/CameraShakes/Spells/BP_ProjectileFireShake.BP_ProjectileFireShake_C")
    (elif (and (`|EnumEquality` _spelltype_2 "Conjure") (`KismetSystemLibrary.IsValidClass` _damagecompanion))
      (`|SpawnActorFromClass` _damagecompanion (`KismetMathLibrary.MakeTransform` (`self.ConjureLocation`)) "Undefined" "MultiplyWithRoot" null null)
      (`AkGameObject.Stop` (`self.Ak_SpellCharge`) :!label _label)
      (`AkGameplayStatics.PostEventAtLocation` _spellfiresound _conjurelocation (`KismetMathLibrary.FindLookAtRotation` _conjurelocation (`self.K2_GetActorLocation`)))
      (switch `int` _id_2
        (:`2`
          (`self.PlayCameraShake` "/Game/Blueprints/CameraShakes/Spells/BP_ConjureCastShake.BP_ConjureCastShake_C"))
        (:`6`
          (`self.PlayCameraShake` "/Game/Blueprints/CameraShakes/Spells/BP_ConjureLightningShake.BP_ConjureLightningShake_C"))
        (:`7`
          (`self.PlayCameraShake` "/Game/Blueprints/CameraShakes/Spells/BP_BloodStrikeShake.BP_BloodStrikeShake_C")))
      (elif (== _id_2 3)
        ;[0 0 0] The only spell in this category is the fire shotgun, so I'm hardcoding logic for it
        (`|SpawnActorFromClass` "/Game/Blueprints/Combat/BP_FireShotgun.BP_FireShotgun_C" (`KismetMathLibrary.MakeTransform` (- (+ (`self.K2_GetActorLocation`) (* _returnvalue 100.0)) (0.0 0.0 90.0)) (`KismetMathLibrary.MakeRotFromX` _returnvalue)) "Undefined" "MultiplyWithRoot" self 50.0 self null)
        (`AkGameObject.Stop` (`self.Ak_SpellCharge`))
        (`AkGameplayStatics.PostEvent` (`.SpellFireSound` (break `Spell` (`JamPlayerState.EquippedSpell` (`self.BP Player State Ref`)))) self)
        (`self.PlayCameraShake` "/Game/Blueprints/CameraShakes/Spells/BP_FireShotgunCastShakeake1.BP_FireShotgunCastShakeake1_C")
        (elif (== (`.ID` (break `Spell` (`JamPlayerState.EquippedSpell` (`self.BP Player State Ref`)))) 7)
          (`|SpawnActorFromClass` (`.DamageCompanion` (break `Spell` (`JamPlayerState.EquippedSpell` (`self.BP Player State Ref`)))) (`KismetMathLibrary.MakeTransform` (- (`self.K2_GetActorLocation`) (0.0 0.0 90.0))) "Undefined" "MultiplyWithRoot" self (`self.GetInstigator`))
          (goto _label)
          (else
            (`self.CastHealSpell`)
            (goto _label)))))))

(fn `GetWorldSaveData`)

(fn `PlayCameraShake`
  (params (Shake :type "CameraShakeBase Class Reference"))
  (`GameplayStatics.PlayWorldCameraShake` Shake (`self.K2_GetActorLocation`) 5.0 500.0))

(fn `PlayNewAKSound`
  (params (`Ak Audio Event` :type "AkAudioEvent Object Reference") (AKComponent :type "AkGameObject Object Reference"))
  (`/Engine/EditorBlueprintResources/StandardMacros.IsValid` AKComponent
    (:`Is Valid`
      (`/Engine/EditorBlueprintResources/StandardMacros.IsValid` (`AkGameObject.AkAudioEvent` AKComponent)
        (:`Is Valid`
          (`AkGameObject.Stop` AKComponent))
        (:`Is Not Valid`
          _))
      (set `AkGameObject.AkAudioEvent` (`local.Ak Audio Event`) (`local.AKComponent`))
      (`AkGameObject.PostAssociatedAkEvent` :`self` (`local.AKComponent`)))))

(fn `RemoveSpellChargeWidget`
  (bind _spellchargewidget (`self.SpellChargeWidget`))
  (`/Engine/EditorBlueprintResources/StandardMacros.IsValid` _spellchargewidget
    (:`Is Valid`
      (`Widget.RemoveFromParent` _spellchargewidget))))

(fn `SetHealthWidget`
  (bind _attributes (`self.Attributes`))
  (`/Game/UI/Common/Widgets/HUD/WB_MainHUD.UpdateHealth` (`/Game/Player/BP_JamPlayerState.HUDRef` (`self.BP Player State Ref`)) (`KismetMathLibrary.SafeDivide` (`AttributesComponent.Health` _attributes) (`AttributesComponent.MaxHealth` _attributes))))

(fn `SetManaWidget`
  (bind _attributes (`self.Attributes`))
  (`/Game/UI/Common/Widgets/HUD/WB_MainHUD.UpdateMana` (`/Game/Player/BP_JamPlayerState.HUDRef` (`self.BP Player State Ref`)) (`KismetMathLibrary.SafeDivide` (`AttributesComponent.Mana` _attributes) (`AttributesComponent.MaxMana` _attributes))))

(fn `SetPotionsWidget`
  (if (`self.hasRedPotion`)
    (`Widget.SetRenderOpacity` (`/Game/UI/Common/Widgets/HUD/WB_MainHUD.RedPotion` (`/Game/Player/BP_JamPlayerState.HUDRef` (`self.BP Player State Ref`))) 1.0))
  (if (`self.hasBlackPotion`)
    (`Widget.SetRenderOpacity` (`/Game/UI/Common/Widgets/HUD/WB_MainHUD.BlackPotion` (`/Game/Player/BP_JamPlayerState.HUDRef` (`self.BP Player State Ref`))) 1.0))
  (if (`self.hasWhitePotion`)
    (`Widget.SetRenderOpacity` (`/Game/UI/Common/Widgets/HUD/WB_MainHUD.WhitePotion` (`/Game/Player/BP_JamPlayerState.HUDRef` (`self.BP Player State Ref`))) 1.0)))

(fn `SetReferences`
  (set `self.BP Player State Ref` (`/Game/Blueprints/BFL_CommonFunctions.GetPlayerStateRef`))
  (set `self.Player Controller Ref` (`/Game/Blueprints/BFL_CommonFunctions.GetPlayerControllerRef`))
  (bind _outactors (`GameplayStatics.GetAllActorsOfClass` "/Game/Blueprints/BP_SpellLock.BP_SpellLock_C"))
  (set `self.CrystalLocks` _outactors)
  (bind _outactors_2 (`GameplayStatics.GetAllActorsOfClass` "/Game/Blueprints/BP_Door.BP_Door_C"))
  (set `self.UnlockableDoors` _outactors_2)
  (set `self.ReferencesSet` true))

(fn `StartSpell`
  (set `self.SpellCancelled` false)
  (set `self.FiredProjectile` false)
  (set `self.SpellChargeProgress` 0.0)
  (set `CharacterMovementComponent.MaxWalkSpeed` (`self.ChargingSpellWalkSpeed`) (`self.CharacterMovement`))
  (switch `ESpellType` (`self.CurrentSpell`)
    (:`TwoHanded`
      (set `self.2hIsCharging` true)
      (set `self.2hFiredProjectile` false))
    (:`Beam`
      (set `self.isCharging` true :!label _label))
    (:`Projectile`
      (goto _label))
    (:`Conjure`
      (goto _label))))

(fn `UpdateDashWidget`
  (`/Game/UI/Common/Widgets/HUD/WB_DashIndicator.SetProgressBarPercent` (`/Game/UI/Common/Widgets/HUD/WB_MainHUD.WB_DashIndicator` (`/Game/Player/BP_JamPlayerState.HUDRef` (`self.BP Player State Ref`))) (`KismetMathLibrary.SafeDivide` (`KismetSystemLibrary.K2_GetTimerElapsedTimeHandle` (`self.FirstDashCooldownTimerHandle`)) (`self.DashCooldownDuration`))))

(fn `UserConstructionScript`
  (`SceneComponent.K2_AttachToComponent` (`self.IdleParticleEffect`) (`self.SkeletalMesh`) "HandProjectileSocket" "SnapToTarget" "SnapToTarget" "SnapToTarget" true)
  (`SceneComponent.K2_AttachToComponent` (`self.L_IdleParticleEffect`) (`self.SkeletalMesh`) "L_ProjectileSocket" "SnapToTarget" "SnapToTarget" "SnapToTarget" true))