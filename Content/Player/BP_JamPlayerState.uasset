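; BP_JamPlayerState is a player state that stores the equipped spell and applies it to the player character.
; After a short BeginPlay delay it caches character, controller and main HUD references, taking the HUD from the master widget's active stack entry.
; SetEquippedSpell copies spell type and two-handed flag to the character, then sets or clears idle particles and Wwise idle sound.
; Two-handed spells mirror the particle onto the left hand.
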(event `self.ReceiveBeginPlay`
  (`KismetSystemLibrary.Delay` 0.2)
  (`self.SetReferences`))

(fn `SetEquippedSpell`
  (params (SpellToEquip :type "Spell Structure"))
  (bind _player_character_ref (`self.Player Character Ref`))
  (bind (_id _name _spelltype _icon _description _isvalid _istwohanded _chargetime _idleparticleeffect) (break `Spell` (`self.EquippedSpell`)))
  (bind (_id_2 _name_2 _spelltype_2 _icon_2 _description_2 _isvalid_2 _istwohanded_2 _chargetime_2 _idleparticleeffect_2 _projectileclass _basedamage _manacost _spellidlesound) (break `Spell` (`self.EquippedSpell`)))
  (bind _l_idleparticleeffect (`/Game/Player/BP_JamPlayerCharacter.L_IdleParticleEffect` (`self.Player Character Ref`)))
  (bind _l_idleparticleeffect_2 (`/Game/Player/BP_JamPlayerCharacter.L_IdleParticleEffect` (`self.Player Character Ref`)))
  (bind _l_idleparticleeffect_3 (`/Game/Player/BP_JamPlayerCharacter.L_IdleParticleEffect` (`self.Player Character Ref`)))
  (bind _l_idleparticleeffect_4 (`/Game/Player/BP_JamPlayerCharacter.L_IdleParticleEffect` (`self.Player Character Ref`)))
  (bind _ak_spellidle (`/Game/Player/BP_JamPlayerCharacter.AK_SpellIdle` (`self.Player Character Ref`)))
  (bind _output_get (set `self.EquippedSpell` SpellToEquip))
  (bind (_id_3 _name_3 _spelltype_3 _icon_3 _description_3 _isvalid_3) (break `Spell` _output_get))
  (set `/Game/Player/BP_JamPlayerCharacter.CurrentSpell` _spelltype_3 (`self.Player Character Ref`))
  (if _isvalid_3
    (bind _output_get_2 (set `/Game/Player/BP_JamPlayerCharacter.2Handed` _istwohanded_2 (`self.Player Character Ref`)))
    (if _output_get_2
      (`|ExecutionSequence`
        (:`then_0`
          (`/Engine/EditorBlueprintResources/StandardMacros.IsValid` _idleparticleeffect_2 :!label _label
            (:`Is Valid`
              ;[0 0 0] Spell data valid, play sound and set idle particle effect
              (`NiagaraComponent.SetAsset` (`/Game/Player/BP_JamPlayerCharacter.IdleParticleEffect` (`self.Player Character Ref`)) _idleparticleeffect_2 true)
              (`NiagaraComponent.SetAsset` _l_idleparticleeffect_2 null true)
              (`ActorComponent.Deactivate` _l_idleparticleeffect_2)
              (`/Game/Player/BP_JamPlayerCharacter.PlayNewAKSound` _player_character_ref _spellidlesound (`/Game/Player/BP_JamPlayerCharacter.AK_SpellIdle` _player_character_ref)))
            (:`Is Not Valid`
              ;[0 0 0] Spell data invalid, clear effects
              (`NiagaraComponent.SetAsset` (`/Game/Player/BP_JamPlayerCharacter.IdleParticleEffect` (`self.Player Character Ref`)) null true :!label _label_2)
              (`NiagaraComponent.SetAsset` _l_idleparticleeffect_4 null true)
              (`ActorComponent.Deactivate` _l_idleparticleeffect_4)
              (`/Engine/EditorBlueprintResources/StandardMacros.IsValid` (`AkGameObject.AkAudioEvent` _ak_spellidle)
                (:`Is Valid`
                  (`AkGameObject.Stop` _ak_spellidle))))))
        (:`then_1`
          ;[0 0 0] Do all the stuff we wanted to do with the right hand, but also add the particle to the left hand
          (`/Engine/EditorBlueprintResources/StandardMacros.IsValid` _idleparticleeffect
            (:`Is Valid`
              (`NiagaraComponent.SetAsset` _l_idleparticleeffect _idleparticleeffect true)
              (`ActorComponent.Activate` _l_idleparticleeffect false))
            (:`Is Not Valid`
              (`NiagaraComponent.SetAsset` _l_idleparticleeffect_3 null true)
              (`ActorComponent.Deactivate` _l_idleparticleeffect_3)))))
      (else
        (goto _label)))
    (else
      (goto _label_2))))

(fn `SetReferences`
  (set `self.Player Character Ref` (`/Game/Blueprints/BFL_CommonFunctions.GetPlayerCharacterRef`))
  (bind _output_get (set `self.Player Controller Ref` (`/Game/Blueprints/BFL_CommonFunctions.GetPlayerControllerRef`)))
  (bind _aswb_main_hud (cast `/Game/UI/Common/Widgets/HUD/WB_MainHUD` (`CommonActivatableWidgetContainerBase.GetActiveWidget` (`/Game/UI/Common/Widgets/WB_MasterWidget.HUD_Stack` (`/Game/Player/BP_JamPlayerController.MasterWidgetRef` _output_get)))))
  (set `self.HUDRef` _aswb_main_hud))

(fn `UserConstructionScript`)