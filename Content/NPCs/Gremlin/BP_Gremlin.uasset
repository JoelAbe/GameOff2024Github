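; Gremlin enemy NPC Blueprint with a melee weapon hitbox and a ragdoll death.
; The construction script attaches the hitbox to the mesh's WeaponSocket, and overlaps damage the player while CanDamage is true.
; Death enables mesh physics, launches the body along the player's projectile direction, clears AIControllerClass and destroys the actor after a delay.
; Taking damage only prints current health here.
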(event `self.OnDamageReceieved`
  (`KismetSystemLibrary.PrintString` (`KismetStringLibrary.Conv_DoubleToString` (`AttributesComponent.Health` (`self.CharacterAttributes`)))))

(event `self.ReceiveBeginPlay`
  (set `self.Player Character Ref` (`/Game/Blueprints/BFL_CommonFunctions.GetPlayerCharacterRef`)))

(event `self.OnDeath`
  (`PrimitiveComponent.SetSimulatePhysics` (`self.Mesh`) true)
  (`PrimitiveComponent.WakeAllRigidBodies` (`self.Mesh`))
  (`PrimitiveComponent.SetCollisionEnabled` (`self.Mesh`) "QueryAndPhysics")
  (`PrimitiveComponent.AddImpulse` (`self.Mesh`) (* (`/Game/Player/BP_JamPlayerCharacter.ProjectileForwardVector` (`self.Player Character Ref`)) 4000.0) "None" true)
  (set `SkeletalMeshComponent.bPauseAnims` true (`self.Mesh`))
  (set `self.AIControllerClass` null)
  (`KismetSystemLibrary.Delay` 5.0)
  (`self.K2_DestroyActor`))

(event `self.Weaponhitbox.OnComponentBeginOverlap`
  (params (OverlappedComponent :type "PrimitiveComponent Object Reference") (OtherActor :type "Actor Object Reference") (OtherComp :type "PrimitiveComponent Object Reference") (OtherBodyIndex :type Integer) (bFromSweep :type Boolean) (SweepResult :type "HitResult Structure (by ref)"))
  (if (and (== OtherActor (`GameplayStatics.GetPlayerCharacter` 0)) (`self.CanDamage`))
    (`GameplayStatics.ApplyDamage` OtherActor (`self.BaseDamage`) (`self.GetInstigatorController`) self)))

(fn `UserConstructionScript`
  (`SceneComponent.K2_AttachToComponent` (`self.Weaponhitbox`) (`self.Mesh`) "WeaponSocket" "KeepRelative" "SnapToTarget" "KeepRelative" true))