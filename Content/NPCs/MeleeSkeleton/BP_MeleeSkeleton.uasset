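; Melee skeleton enemy that damages the player through a box overlap, with its weapon mesh socketed to the skeleton.
; Overlap hits require CanDamage and pass through a DoOnce that a short timer resets to prevent repeat hits.
; Taking damage briefly sets a flag and plays a Wwise sound, while breaking super armor spawns a burst effect and clears the shield.
; Death ragdolls the body along the player's projectile direction, then destroys it after a delay.
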(event `self.OnSuperArmorBroken`
  (`NiagaraFunctionLibrary.SpawnSystemAtLocation` (`self.SuperArmorBreakEffect`) (+ (`SceneComponent.K2_GetComponentLocation` (`self.Mesh`)) (0.0 0.0 200.0)) (struct) (10.76 10.76 11.33))
  (`NiagaraComponent.SetAsset` (`self.SuperArmorShieldEffect`) null true))

(event `self.OnDamageReceieved`
  (set `self.TookDamage` true)
  (if (not (`self.isDead`))
    (`AkGameplayStatics.PostEvent` "/Game/WwiseAudio/DamageDealt.DamageDealt" self)
    (`KismetSystemLibrary.Delay` 0.15)
    (set `self.TookDamage` false)))

(event `self.ReceiveBeginPlay`
  (set `self.DefaultWalkSpeed` 325.0)
  (set `self.Player Character Ref` (`/Game/Blueprints/BFL_CommonFunctions.GetPlayerCharacterRef`)))

(event `self.OnDeath`
  (`PrimitiveComponent.SetSimulatePhysics` (`self.Mesh`) true)
  (`AkGameplayStatics.PostEvent` "/Game/WwiseAudio/SkelHevyDeath.SkelHevyDeath" self)
  (`PrimitiveComponent.WakeAllRigidBodies` (`self.Mesh`))
  (`PrimitiveComponent.SetCollisionEnabled` (`self.Mesh`) "QueryAndPhysics")
  (`PrimitiveComponent.AddImpulse` (`self.Mesh`) (* (`/Game/Player/BP_JamPlayerCharacter.ProjectileForwardVector` (`self.Player Character Ref`)) 4000.0) "None" true)
  (set `SkeletalMeshComponent.bPauseAnims` true (`self.Mesh`))
  (set `self.AIControllerClass` null)
  (`KismetSystemLibrary.Delay` 5.0)
  (`self.K2_DestroyActor`))

(event `self.Box.OnComponentBeginOverlap`
  (params (OverlappedComponent :type "PrimitiveComponent Object Reference") (OtherActor :type "Actor Object Reference") (OtherComp :type "PrimitiveComponent Object Reference") (OtherBodyIndex :type Integer) (bFromSweep :type Boolean) (SweepResult :type "HitResult Structure (by ref)"))
  (if (and (== OtherActor (`GameplayStatics.GetPlayerCharacter` 0)) (`self.CanDamage`))
    ;[0 0 0] Prevents multiple overlaps
    (`KismetSystemLibrary.K2_SetTimerDelegate` (delegate `AllowDamage`) 0.2)
    (`/Engine/EditorBlueprintResources/StandardMacros.DoOnce` false :!label _label
      (:`Completed`
        (`GameplayStatics.ApplyDamage` OtherActor (`self.BaseDamage`) (`self.GetInstigatorController`) self)))))

(event `AllowDamage`
  ;[0 0 0] Prevents multiple overlaps
  (goto _label :!via `Reset`))

(fn `UserConstructionScript`
  (`SceneComponent.K2_AttachToComponent` (`self.WeaponMesh`) (`self.Mesh`) "WeaponSocket" "KeepRelative" "KeepRelative" "KeepRelative" true))