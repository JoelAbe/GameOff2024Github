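; BP_MageNPC is a skeleton mage enemy that fires projectiles at the player from a staff attached to its weapon socket.
; GetPrimeLocation claims the first available prime location from its room manager and writes it to the AI Blackboard.
; FireProjectile spawns and launches a projectile from the staff socket toward the player.
; On death it plays Wwise audio, ragdolls along the player's projectile direction, then destroys itself after a delay.
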(event `self.ReceiveBeginPlay`
  (set `self.DefaultWalkSpeed` 600.0)
  (set `self.Player Character Ref` (`/Game/Blueprints/BFL_CommonFunctions.GetPlayerCharacterRef`)))

(event `self.OnDeath`
  (`PrimitiveComponent.SetSimulatePhysics` (`self.Mesh`) true)
  (`AkGameplayStatics.PostEvent` "/Game/WwiseAudio/SkelMageDeath.SkelMageDeath" self)
  (`PrimitiveComponent.WakeAllRigidBodies` (`self.Mesh`))
  (`PrimitiveComponent.SetCollisionEnabled` (`self.Mesh`) "QueryAndPhysics")
  (set `SkeletalMeshComponent.bPauseAnims` true (`self.Mesh`))
  (`PrimitiveComponent.AddImpulse` (`self.Mesh`) (* (`/Game/Player/BP_JamPlayerCharacter.ProjectileForwardVector` (`self.Player Character Ref`)) 4000.0) "None" true)
  (set `self.AIControllerClass` null)
  (`KismetSystemLibrary.Delay` 5.0)
  (`self.K2_DestroyActor`))

(event `self.OnDamageReceieved`
  (`KismetSystemLibrary.PrintString` (`KismetStringLibrary.Conv_DoubleToString` (`AttributesComponent.Health` (`self.CharacterAttributes`))))
  (if (not (`self.isDead`))
    (`AkGameplayStatics.PostEvent` "/Game/WwiseAudio/DamageDealt.DamageDealt" self)))

(fn `FireProjectile`
  (bind _returnvalue (`SceneComponent.GetSocketLocation` (`self.SKM_SK_MagicStaff`) "ProjectileSocket"))
  (bind _returnvalue_2 (`|SpawnActorFromClass` (`self.ProjectileClass`) (`KismetMathLibrary.MakeTransform` _returnvalue (`KismetMathLibrary.FindLookAtRotation` _returnvalue (`self.K2_GetActorLocation` (`self.PlayerCharacter`)))) "Undefined" "MultiplyWithRoot" self (`self.BaseDamage`) (struct) true (`self.GetInstigator`)))
  (`MagicProjectile.LaunchProjectile` _returnvalue_2)
  (set `self.Attacking` false))

(fn `GetPrimeLocation`
  (bind _roomowner (`self.RoomOwner`))
  (`KismetSystemLibrary.PrintString` (`KismetSystemLibrary.GetDisplayName` _roomowner))
  (bind _asbp_room_manager (cast `/Game/Blueprints/Combat/BP_RoomManager` _roomowner))
  (for _array_element (`/Game/Blueprints/Combat/BP_RoomManager.PrimeLocations` _asbp_room_manager)
    (if (`/Game/Blueprints/Combat/BP_PrimeLocation.isAvailable` _array_element)
      (`BlackboardComponent.SetValueAsVector` (`AIController.Blackboard` (`self.AIController`)) "PrimeLocation" (`self.K2_GetActorLocation` _array_element))
      (set `/Game/Blueprints/Combat/BP_PrimeLocation.isAvailable` false _array_element)
      (set `self.FoundLocation` true)
      (break)))
  (if (not (`self.FoundLocation`))
    (`BlackboardComponent.ClearValue` (`AIController.Blackboard` (`self.AIController`)) "PrimeLocation")))

(fn `UserConstructionScript`
  (`SceneComponent.K2_AttachToComponent` (`self.SKM_SK_MagicStaff`) (`self.Mesh`) "WeaponSocket" "KeepRelative" "KeepRelative" "KeepRelative" true))