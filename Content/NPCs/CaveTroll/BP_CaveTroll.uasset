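; Cave troll final boss that enters its waiting state when the Boss-tagged combat trigger fires and flags the player's victory on death.
; Attack events play montages with Wwise audio, while weapon overlaps deal melee damage to the player.
; Montage notifies add a three-way arcane blast to HammerSwing and a trace-grounded fire shotgun to BigSlam.
; Armor meshes follow the body through leader pose, and breaking super armor swaps the shield for a burst effect.
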(event `self.OnDeath`
  (`self.StopAnimMontage` (`self.GetCurrentMontage`))
  (`PrimitiveComponent.SetCollisionEnabled` (`self.WeaponCollision`) "NoCollision")
  (`KismetSystemLibrary.Delay` 5.0)
  (set `SkeletalMeshComponent.bPauseAnims` true (`self.Mesh`))
  (set `self.AIControllerClass` null)
  (set `/Game/Player/BP_JamPlayerCharacter.beatFinalBoss?` true (`/Game/Blueprints/BFL_CommonFunctions.GetPlayerCharacterRef`)))

(event `self.ReceiveBeginPlay`
  (bind _outactors (`GameplayStatics.GetAllActorsOfClassWithTag` "/Game/Blueprints/Combat/BP_CombatTrigger.BP_CombatTrigger_C" "Boss"))
  (add `/Game/Blueprints/Combat/BP_CombatTrigger.OnBossCombatTriggered` (`|GetArrayItem` _outactors) (delegate `OnBossCombatTriggered_Event`)))

(event `OnBossCombatTriggered_Event`
  (`self.SetStateWaiting`))

(event `self.OnSuperArmorBroken`
  (`NiagaraFunctionLibrary.SpawnSystemAtLocation` (`self.SuperArmorBreakEffect`) (+ (`SceneComponent.K2_GetComponentLocation` (`self.Mesh`)) (0.0 0.0 200.0)) (struct) (10.76 10.76 11.33))
  (`NiagaraComponent.SetAsset` (`self.SuperArmorShieldEffect`) null true))

(event `FastHammerSwing`
  ;[0 0 0] Attack 2
  (`|PlayMontage` (`self.Mesh`) "/Game/CaveTrollMedium/Animation/Troll_Attack2Fast_Montage.Troll_Attack2Fast_Montage"
    (:`then`
      (`AkGameplayStatics.PostEventAtLocation` "/Game/WwiseAudio/TrollDA2.TrollDA2" (`self.K2_GetActorLocation`) (`KismetMathLibrary.Conv_VectorToRotator` (`self.GetActorForwardVector`))))))

(event `HammerSwing`
  ;[0 0 0] Attack1
  (`|PlayMontage` (`self.Mesh`) "/Game/CaveTrollMedium/Animation/TrollAttack1_Montage.TrollAttack1_Montage"
    (:`then`
      (`AkGameplayStatics.PostEventAtLocation` "/Game/WwiseAudio/TrollDA1.TrollDA1" (`self.K2_GetActorLocation`) (`KismetMathLibrary.Conv_VectorToRotator` (`self.GetActorForwardVector`))))
    (:`OnNotifyBegin`
      (`self.FireScattershot`))))

(event `SlowHammerSwing`
  ;[0 0 0] Attack3
  (`|PlayMontage` (`self.Mesh`) "/Game/CaveTrollMedium/Animation/Troll_Attack3_Slow_Montage.Troll_Attack3_Slow_Montage"
    (:`then`
      (`AkGameplayStatics.PostEventAtLocation` "/Game/WwiseAudio/TrollDA3.TrollDA3" (`self.K2_GetActorLocation`) (`KismetMathLibrary.Conv_VectorToRotator` (`self.GetActorForwardVector`))))))

(event `BigSlam`
  ;[0 0 0] Attack 4
  (`|PlayMontage` (`self.Mesh`) "/Game/CaveTrollMedium/Animation/Troll_Attack4_BigSlam_Montage.Troll_Attack4_BigSlam_Montage"
    (:`then`
      (`AkGameplayStatics.PostEventAtLocation` "/Game/WwiseAudio/TrollSlam.TrollSlam" (`self.K2_GetActorLocation`) (`KismetMathLibrary.Conv_VectorToRotator` (`self.GetActorForwardVector`))))
    (:`OnNotifyBegin`
      (`self.FireBigSlam`)
      (`AkGameplayStatics.PostEventAtLocation` "/Game/WwiseAudio/VortexCast.VortexCast" (`self.K2_GetActorLocation`) (`KismetMathLibrary.Conv_VectorToRotator` (`self.GetActorForwardVector`))))))

(event `self.WeaponCollision.OnComponentBeginOverlap`
  (params (OverlappedComponent :type "PrimitiveComponent Object Reference") (OtherActor :type "Actor Object Reference") (OtherComp :type "PrimitiveComponent Object Reference") (OtherBodyIndex :type Integer) (bFromSweep :type Boolean) (SweepResult :type "HitResult Structure (by ref)"))
  (if (and (== OtherActor (`GameplayStatics.GetPlayerCharacter` 0)) (`self.CanDamage`))
    (`GameplayStatics.ApplyDamage` OtherActor (`self.MeleeDamage`) (`self.GetInstigatorController`) self)))

(event `Death`
  ;[0 0 0] Troll death
)

(event `Surprise`
  ;[0 0 0] Surprise!
  (`|PlayMontage` (`self.Mesh`) "/Game/CaveTrollMedium/Animation/Troll_Surprise_Montage.Troll_Surprise_Montage"))

(fn `CalculateFireShotgunLocation`
  (returns (SpawnLocation :type "Vector Structure"))
  (bind _returnvalue (- (`SceneComponent.K2_GetComponentLocation` (`self.Mesh`)) (0.0 0.0 25.0)))
  (bind _outhit (`KismetSystemLibrary.LineTraceSingle` _returnvalue (+ _returnvalue (* (`self.GetActorForwardVector`) 200.0)) "TraceTypeQuery1"))
  (bind (_bblockinghit _binitialoverlap _time _distance _location _impactpoint _normal _impactnormal _physmat _hitactor _hitcomponent _hitbonename _bonename _hititem _elementindex _faceindex _tracestart _traceend) (`GameplayStatics.BreakHitResult` _outhit))
  (bind _outhit_2 (`KismetSystemLibrary.LineTraceSingle` _traceend (+ (* (`KismetMathLibrary.Vector_Down`) 500.0) _traceend) "TraceTypeQuery1"))
  (return (+ (`.ImpactPoint` (`GameplayStatics.BreakHitResult` _outhit_2)) (0.0 0.0 10.0))))

(fn `FireBigSlam`
  (bind _spawnlocation (`self.CalculateFireShotgunLocation`))
  (`|SpawnActorFromClass` "/Game/Blueprints/Combat/BP_FireShotgun.BP_FireShotgun_C" (`KismetMathLibrary.MakeTransform` _spawnlocation (`KismetMathLibrary.Conv_VectorToRotator` (`self.GetActorForwardVector`)) (2.0 1.0 1.0)) "Undefined" "MultiplyWithRoot" self (`self.FireShotgunDamage`) self null))

(fn `FireScattershot`
  (bind (_centerlocation _leftlocation _rightlocation _centerrotation _leftrotation _rightrotation) (`self.GetScattershotRotations`))
  (`|ExecutionSequence`
    (:`then_0`
      (bind _returnvalue (`|SpawnActorFromClass` "/Game/Blueprints/Projectiles/PlayerProjectiles/BP_ArcaneBlast.BP_ArcaneBlast_C" (`KismetMathLibrary.MakeTransform` _centerlocation _centerrotation) "Undefined" "MultiplyWithRoot" null (`self.ArcaneBlastDamage`) (struct) true null))
      (`MagicProjectile.LaunchProjectile` _returnvalue))
    (:`then_1`
      (bind _returnvalue_2 (`|SpawnActorFromClass` "/Game/Blueprints/Projectiles/PlayerProjectiles/BP_ArcaneBlast.BP_ArcaneBlast_C" (`KismetMathLibrary.MakeTransform` _leftlocation _leftrotation) "Undefined" "MultiplyWithRoot" null (`self.ArcaneBlastDamage`) (struct) true null))
      (`MagicProjectile.LaunchProjectile` _returnvalue_2))
    (:`then_2`
      (bind _returnvalue_3 (`|SpawnActorFromClass` "/Game/Blueprints/Projectiles/PlayerProjectiles/BP_ArcaneBlast.BP_ArcaneBlast_C" (`KismetMathLibrary.MakeTransform` _rightlocation _rightrotation) "Undefined" "MultiplyWithRoot" null (`self.ArcaneBlastDamage`) (struct) true null))
      (`MagicProjectile.LaunchProjectile` _returnvalue_3))))

(fn `GetScattershotRotations`
  (returns (CenterLocation :type "Vector Structure") (LeftLocation :type "Vector Structure") (RightLocation :type "Vector Structure") (CenterRotation :type "Rotator Structure") (LeftRotation :type "Rotator Structure") (RightRotation :type "Rotator Structure"))
  (locals (LeftRotatorOffset :type "Rotator Structure" :default (struct :`Yaw` -15.0)) (RightRotatorOffset :type "Rotator Structure" :default (struct :`Yaw` 15.0)) (CenterSpawnLocation :type "Vector Structure") (LeftSpawnLocation :type "Vector Structure") (RightSpawnLocation :type "Vector Structure"))
  (bind (_leftrotatoroffset_roll _leftrotatoroffset_pitch _leftrotatoroffset_yaw) (`KismetMathLibrary.BreakRotator` (`local.LeftRotatorOffset`)))
  (bind (_rightrotatoroffset_roll _rightrotatoroffset_pitch _rightrotatoroffset_yaw) (`KismetMathLibrary.BreakRotator` (`local.RightRotatorOffset`)))
  (bind (_returnvalue_roll _returnvalue_pitch _returnvalue_yaw) (`KismetMathLibrary.BreakRotator` (`KismetMathLibrary.MakeRotFromX` (`self.GetActorForwardVector`))))
  (bind (_returnvalue_roll_2 _returnvalue_pitch_2 _returnvalue_yaw_2) (`KismetMathLibrary.BreakRotator` (`KismetMathLibrary.MakeRotFromX` (`self.GetActorForwardVector`))))
  (set `local.CenterSpawnLocation` (+ (`self.K2_GetActorLocation`) (* (`self.GetActorForwardVector`) 200.0)))
  (set `local.LeftSpawnLocation` (- (`local.CenterSpawnLocation`) (* (`self.GetActorRightVector`) 100.0)))
  (set `local.RightSpawnLocation` (+ (`local.CenterSpawnLocation`) (* (`self.GetActorRightVector`) 100.0)))
  (return (`local.CenterSpawnLocation`) (`local.LeftSpawnLocation`) (`local.RightSpawnLocation`) (`KismetMathLibrary.MakeRotFromX` (`self.GetActorForwardVector`)) (`KismetMathLibrary.MakeRotator` (+ _returnvalue_roll_2 _leftrotatoroffset_roll) (+ _returnvalue_pitch_2 _leftrotatoroffset_pitch) (+ _returnvalue_yaw_2 _leftrotatoroffset_yaw)) (`KismetMathLibrary.MakeRotator` (+ _returnvalue_roll _rightrotatoroffset_roll) (+ _returnvalue_pitch _rightrotatoroffset_pitch) (+ _returnvalue_yaw _rightrotatoroffset_yaw))))

(fn `UserConstructionScript`
  (`SceneComponent.K2_AttachToComponent` (`self.Weapon`) (`self.Mesh`) "WeaponSocket" "SnapToTarget" "SnapToTarget" "KeepRelative" true)
  (`SkinnedMeshComponent.SetLeaderPoseComponent` (`self.Belt`) (`self.Mesh`) false false)
  (`SkinnedMeshComponent.SetLeaderPoseComponent` (`self.Shoulder`) (`self.Mesh`) false false)
  (`SkinnedMeshComponent.SetLeaderPoseComponent` (`self.Corpse`) (`self.Mesh`) false false)
  (`SkinnedMeshComponent.SetLeaderPoseComponent` (`self.Helmet`) (`self.Mesh`) false false)
  (`SkinnedMeshComponent.SetLeaderPoseComponent` (`self.LegArmor`) (`self.Mesh`) false false))